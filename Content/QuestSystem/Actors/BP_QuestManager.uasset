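; Quest manager actor that tracks active, completed and failed quest actors and keeps the journal, quest list and minimap in sync.
; Talk, item-found and kill events advance matching goals, deferring quest-completing ones until iteration ends.
; The selected subgoal spawns a goal marker driving distance text and a direction arrow.
; Quests spawn by class without duplicates, reload from GameInstance data, and grant experience and regional prestige on completion.
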(event `OnTalkToNPC`
  (params (NPCClass :type "/Game/Blueprint/AI_With_Markovs_chain/BP_MasterNPC Class Reference") (NPCid :type Integer) (NPCName :type Text))
  ;[1 1 1] Выполнение квеста на разговор
  (`KismetArrayLibrary.Array_Clear` (`self.IndecesToCompleteLater`))
  (for _array_element (`self.CurrentQuestActors`)
    (for (_array_element_2 _array_index) (`/Game/Blueprint/QuestActors/BP_MasterQuest.CurrentGoals` _array_element)
      (bind (_type _customgoal_ _goaltext _addition _amounttohunt _goalclass _taggoal _npcname _goalid _goallocation _useradius_ _radius _circlecolour _updatequestdesc_ _updateddescription _subgoalindecies _failmeansquestfail_ _completequest_) (break `/Game/QuestSystem/Structure/S_GoalInfo` _array_element_2))
      (if (and (`|EnumEquality` _type "NewEnumerator3") (== _goalclass NPCClass) (`KismetTextLibrary.EqualEqual_TextText` _npcname NPCName))
        (if _completequest_
          (bind _output (`|GetArrayItem` (`/Game/Blueprint/QuestActors/BP_MasterQuest.CurrentGoalIndecies` _array_element) _array_index))
          (`KismetArrayLibrary.Array_Add` (`self.IndecesToCompleteLater`) (make `/Game/QuestSystem/Structure/S_IndexToComplete` _array_element _output))
          (else
            (`/Game/Blueprint/QuestActors/BP_MasterQuest.CompleteSubGoal` _array_element _output false))))))
  (`self.CompleteGoals`))

(event `OnObjectFound`
  (params (FoundObject :type "/Game/Blueprint/Props/Blueprints/BP_InteractiveObj Class Reference"))
  ;[1 1 1] Выполнение квеста на поиск предмета
  (`KismetArrayLibrary.Array_Clear` (`self.IndecesToCompleteLater`))
  (set `self.Found Object` FoundObject)
  (for _array_element (`self.CurrentQuestActors`)
    (for (_array_element_2 _array_index) (`/Game/Blueprint/QuestActors/BP_MasterQuest.CurrentGoals` _array_element)
      (bind (_type _customgoal_ _goaltext _addition _amounttohunt _goalclass _taggoal _npcname _goalid _goallocation _useradius_ _radius _circlecolour _updatequestdesc_ _updateddescription _subgoalindecies _failmeansquestfail_ _completequest_) (break `/Game/QuestSystem/Structure/S_GoalInfo` _array_element_2))
      (if (and (`|EnumEquality` _type "NewEnumerator2") (== _goalclass (`self.Found Object`)))
        (if _completequest_
          (bind _output (`|GetArrayItem` (`/Game/Blueprint/QuestActors/BP_MasterQuest.CurrentGoalIndecies` _array_element) _array_index))
          (`KismetArrayLibrary.Array_Add` (`self.IndecesToCompleteLater`) (make `/Game/QuestSystem/Structure/S_IndexToComplete` _array_element _output))
          (else
            (`/Game/Blueprint/QuestActors/BP_MasterQuest.CompleteSubGoal` _array_element _output false))))))
  (`self.CompleteGoals`))

(event `OnEnemyKilled`
  (params (Class :type "/Game/Blueprint/AI_With_Markovs_chain/BP_MasterNPC Class Reference"))
  ;[1 1 1] Выполнение квеста на убийство
  (`KismetArrayLibrary.Array_Clear` (`self.IndecesToCompleteLater`))
  (set `self.killedenemy` Class)
  (for _array_element (`self.CurrentQuestActors`)
    (for (_array_element_2 _array_index) (`/Game/Blueprint/QuestActors/BP_MasterQuest.CurrentGoals` _array_element)
      (bind (_type _customgoal_ _goaltext _addition _amounttohunt _goalclass _taggoal _npcname _goalid _goallocation _useradius_ _radius _circlecolour _updatequestdesc_ _updateddescription _subgoalindecies _failmeansquestfail_ _completequest_) (break `/Game/QuestSystem/Structure/S_GoalInfo` _array_element_2))
      (if (and (`|EnumEquality` _type "NewEnumerator1") (== _goalclass (`self.killedenemy`)))
        (bind _returnvalue (+ (`|GetArrayItem` (`/Game/Blueprint/QuestActors/BP_MasterQuest.CurretHuntedAmounts` _array_element) _array_index) 1))
        (if (>= _returnvalue _amounttohunt)
          (if _completequest_
            (bind _output (`|GetArrayItem` (`/Game/Blueprint/QuestActors/BP_MasterQuest.CurrentGoalIndecies` _array_element) _array_index))
            (`KismetArrayLibrary.Array_Add` (`self.IndecesToCompleteLater`) (make `/Game/QuestSystem/Structure/S_IndexToComplete` _array_element _output))
            (else
              (`/Game/Blueprint/QuestActors/BP_MasterQuest.CompleteSubGoal` _array_element _output false)))
          (else
            (`KismetArrayLibrary.Array_Set` (`/Game/Blueprint/QuestActors/BP_MasterQuest.CurretHuntedAmounts` _array_element) _array_index _returnvalue)
            (`/Game/QuestSystem/Widgets/W_SubGoalWidget.Update` (`|GetArrayItem` (`/Game/QuestSystem/Widgets/W_QuestWidget.SubGoladWidget` (`/Game/Blueprint/QuestActors/BP_MasterQuest.QuestWidget` _array_element)) _array_index))
            (if (`/Game/Blueprint/QuestActors/BP_MasterQuest.SelectedInJournal` _array_element)
              (`/Game/QuestSystem/Widgets/W_QuestJournal.GenerateSubGoals` (`/Game/QuestSystem/Widgets/W_MainWidget.W_QuestJournal` (`self.MainWidget`)))))))))
  (`self.CompleteGoals`))

(event `OnSwitchSubQuest`
  (bind _currentquest (`self.CurrentQuest`))
  (bind _mainwidget (`self.MainWidget`))
  (bind _outactors (`GameplayStatics.GetAllActorsOfClass` "/Game/Blueprint/QuestActors/BP_GoalActor.BP_GoalActor_C"))
  (`self.K2_DestroyActor` _outactors)
  (bind _output_get (set `self.CurrentSubGoal` (`|GetArrayItem` (`.SubGoals_24_0D709B5D4238C144508DD1B2EDE066F5` (break `/Game/QuestSystem/Structure/S_QuestInfo` (`/Game/Blueprint/QuestActors/BP_MasterQuest.QuestInfo` _currentquest))) (`/Game/Blueprint/QuestActors/BP_MasterQuest.SelectedSubGoalIndex` _currentquest))))
  (bind (_type _customgoal_ _goaltext _addition _amounttohunt _goalclass _taggoal _npcname _goalid _goallocation _useradius_ _radius _circlecolour) (break `/Game/QuestSystem/Structure/S_GoalInfo` _output_get))
  (bind (_haslocation_ _location) (break `/Game/QuestSystem/Structure/S_GoalLocation` _goallocation))
  (if _haslocation_
    (bind _returnvalue (`|SpawnActorFromClass` "/Game/Blueprint/QuestActors/BP_GoalActor.BP_GoalActor_C" (`KismetMathLibrary.MakeTransform` _location) "AlwaysSpawn" "OverrideRootScale" null _useradius_ _radius _circlecolour null))
    (set `self.CurrentGoalACtor` _returnvalue)
    (bind _output_get_2 (set `self.CurrentDistance` (`self.DistanceToGoal`)))
    (`TextBlock.SetText` (`/Game/QuestSystem/Widgets/W_MainWidget.DistanceText` (`self.MainWidget`)) (`KismetTextLibrary.Conv_IntToText` _output_get_2 false false))
    (`self.UpdateDirectionArrow?`)
    (`Widget.SetVisibility` (`/Game/QuestSystem/Widgets/W_MainWidget.DistanceBorder` _mainwidget) "HitTestInvisible")
    (`Widget.SetVisibility` (`/Game/QuestSystem/Widgets/W_MiniMap.DirectionArrow` (`/Game/QuestSystem/Widgets/W_MainWidget.W_MiniMap` _mainwidget)) (select `bool` (> (`self.CurrentDistance`) (`self.ShowDirectionArrowAmount`)) :`false` "Hidden" :`true` "HitTestInvisible" :!type "ESlateVisibility Enum"))
    (else
      (set `self.CurrentGoalACtor` null)
      (`Widget.SetVisibility` (`/Game/QuestSystem/Widgets/W_MainWidget.DistanceBorder` (`self.MainWidget`)) "Hidden")
      (`Widget.SetVisibility` (`/Game/QuestSystem/Widgets/W_MiniMap.DirectionArrow` (`/Game/QuestSystem/Widgets/W_MainWidget.W_MiniMap` (`self.MainWidget`))) "Hidden"))))

(event `OnPlayerMoveS`
  ;[1 1 1] Обновляем стрелку указывающую на область квеста
  (`/Engine/EditorBlueprintResources/StandardMacros.IsValid` (`self.CurrentGoalACtor`)
    (:`Is Valid`
      (bind _output_get (set `self.CurrentDistance` (`self.DistanceToGoal`)))
      (`TextBlock.SetText` (`/Game/QuestSystem/Widgets/W_MainWidget.DistanceText` (`self.MainWidget`)) (`KismetTextLibrary.Conv_IntToText` _output_get false false))
      (`/Engine/EditorBlueprintResources/StandardMacros.CompareInt` (`self.CurrentDistance`) (`self.ShowDirectionArrowAmount`)
        (:`>`
          _)
        (:`==`
          _)
        (:`<`
          (`/Engine/EditorBlueprintResources/StandardMacros.DoOnce` false :!label _label
            (:`Completed`
              (`Widget.SetVisibility` (`/Game/QuestSystem/Widgets/W_MiniMap.DirectionArrow` (`/Game/QuestSystem/Widgets/W_MainWidget.W_MiniMap` (`self.MainWidget`))) "Hidden")
              (goto _label_2 :!via `Reset`)))))
      (`self.UpdateDirectionArrow?`)
      (`/Engine/EditorBlueprintResources/StandardMacros.DoOnce` false :!label _label_2
        (:`Completed`
          (`Widget.SetVisibility` (`/Game/QuestSystem/Widgets/W_MiniMap.DirectionArrow` (`/Game/QuestSystem/Widgets/W_MainWidget.W_MiniMap` (`self.MainWidget`))) "HitTestInvisible")
          (goto _label :!via `Reset`))))))

(event `self.ReceiveBeginPlay`
  ;[1 1 1] СОхранение ссылки на гейм инстанс
  (bind _asbp_game_instance_not_working (cast `/Game/Blueprint/LevelBP/BP/BP_GameInstanceNotWorking` (`GameplayStatics.GetGameInstance`)))
  (set `self.As BP Game Instance Not Working` _asbp_game_instance_not_working))

(event `LoadQuests`
  (bind _allquestclasses (`self.AllQuestClasses`))
  (bind _loadedquest (`self.LoadedQuest`))
  (bind _mainwidget (`self.MainWidget`))
  (bind _loadedquest_2 (`self.LoadedQuest`))
  (bind _mainwidget_2 (`self.MainWidget`))
  (bind _mainwidget_3 (`self.MainWidget`))
  (bind _currentstate (`/Game/Blueprint/QuestActors/BP_MasterQuest.CurrentState` _loadedquest_2))
  (bind _w_questjournal (`/Game/QuestSystem/Widgets/W_MainWidget.W_QuestJournal` _mainwidget_2))
  (`KismetArrayLibrary.Array_Clear` (`self.AllQuestClasses`))
  (`KismetArrayLibrary.Array_Clear` (`self.CurrentQuestActors`))
  (`KismetArrayLibrary.Array_Clear` (`self.CompletedQuestActors`))
  (`KismetArrayLibrary.Array_Clear` (`self.FailedQuestActors`))
  (`PanelWidget.ClearChildren` (`/Game/QuestSystem/Widgets/W_QuestCategory.QuestBox` (`/Game/QuestSystem/Widgets/W_QuestJournal.CatCur` _w_questjournal)))
  (`PanelWidget.ClearChildren` (`/Game/QuestSystem/Widgets/W_QuestCategory.QuestBox` (`/Game/QuestSystem/Widgets/W_QuestJournal.CatFail` _w_questjournal)))
  (`PanelWidget.ClearChildren` (`/Game/QuestSystem/Widgets/W_QuestCategory.QuestBox` (`/Game/QuestSystem/Widgets/W_QuestJournal.CatComp` _w_questjournal)))
  (`Widget.SetVisibility` (`/Game/QuestSystem/Widgets/W_QuestJournal.QuestDetailsBox` _w_questjournal) "Hidden")
  (`PanelWidget.ClearChildren` (`/Game/QuestSystem/Widgets/W_MainWidget.QuestList` _mainwidget_2))
  (for _array_element (`/Game/Blueprint/LevelBP/BP/BP_GameInstanceNotWorking.LoadSavedQuests` (`self.As BP Game Instance Not Working`))
    (bind (_questclass _currentactive_ _currentgoalindeces _huntamount _selectedgoalindex _currentgoals _completedgoals _membervar _currentstate_2 _currentdesc) (break `/Game/QuestSystem/Structure/S_SavedQuest` _array_element))
    (if (`KismetArrayLibrary.Array_Contains` _allquestclasses _questclass)
      (`KismetSystemLibrary.PrintString` "Такой квест уже существует, надо обновлять список " true true (struct :`R` 1.0 :`B` 0.078669 :`A` 1.0) 999.0)
      (else
        (`KismetArrayLibrary.Array_Add` _allquestclasses _questclass)
        (bind _returnvalue (`|SpawnActorFromClass` _questclass (`KismetMathLibrary.MakeTransform` (0.0 0.0 0.0)) "Undefined" "OverrideRootScale" null self null null))
        (set `self.LoadedQuest` _returnvalue)
        (`/Engine/EditorBlueprintResources/StandardMacros.IsValid` (`self.LoadedQuest`)
          (:`Is Valid`
            (set `/Game/Blueprint/QuestActors/BP_MasterQuest.CurrentGoalIndecies` _currentgoalindeces _loadedquest_2)
            (set `/Game/Blueprint/QuestActors/BP_MasterQuest.CurretHuntedAmounts` _huntamount _loadedquest_2)
            (set `/Game/Blueprint/QuestActors/BP_MasterQuest.SelectedSubGoalIndex` _selectedgoalindex _loadedquest_2)
            (set `/Game/Blueprint/QuestActors/BP_MasterQuest.CurrentGoals` _currentgoals _loadedquest_2)
            (set `/Game/Blueprint/QuestActors/BP_MasterQuest.CompletedSubGoals` _completedgoals _loadedquest_2)
            (set `/Game/Blueprint/QuestActors/BP_MasterQuest.CurrentState` _currentstate_2 _loadedquest_2)
            (set `/Game/Blueprint/QuestActors/BP_MasterQuest.CurentDesc` _currentdesc _loadedquest_2)
            (`KismetArrayLibrary.Array_Add` (select `/Game/QuestSystem/Enums/E_QuestStates` _currentstate :`NewEnumerator0` (`self.CurrentQuestActors`) :`NewEnumerator1` (`self.CompletedQuestActors`) :`NewEnumerator2` (`self.FailedQuestActors`)) _loadedquest_2)
            (`/Game/QuestSystem/Widgets/W_QuestJournal.AddEntry` (`/Game/QuestSystem/Widgets/W_MainWidget.W_QuestJournal` _mainwidget) _loadedquest_2)
            (if (`|EnumEquality` _currentstate "NewEnumerator0")
              (bind _questwidget (`/Game/QuestSystem/Widgets/W_MainWidget.AddQuestToList` _mainwidget _loadedquest_2))
              (set `/Game/Blueprint/QuestActors/BP_MasterQuest.QuestWidget` _questwidget _loadedquest)
              (`/Game/QuestSystem/Widgets/W_QuestWidget.UpdateQuest` _questwidget)
              (if _currentactive_
                (`self.SelectNewQuest` _loadedquest (`|GetArrayItem` (`/Game/QuestSystem/Widgets/W_QuestWidget.SubGoladWidget` _questwidget) (`KismetArrayLibrary.Array_Find` (`/Game/Blueprint/QuestActors/BP_MasterQuest.CurrentGoalIndecies` _loadedquest) (`/Game/Blueprint/QuestActors/BP_MasterQuest.SelectedSubGoalIndex` _loadedquest))) true)
                (if (`/Game/QuestSystem/Widgets/W_MainWidget.SlideOut?` _mainwidget_3)
                  (`UserWidget.PlayAnimation` _mainwidget_3 (`/Game/QuestSystem/Widgets/W_MainWidget.SlideOut` _mainwidget_3) 0.0 1 "Reverse" 1.0 false)
                  (set `/Game/QuestSystem/Widgets/W_MainWidget.SlideOut?` false _mainwidget_3))))))))))

(fn `AddNewquest`
  (params (QuestClas :type "/Game/Blueprint/QuestActors/BP_MasterQuest Class Reference") (`DirectlyStaert?` :type Boolean))
  (returns (Succ :type Boolean))
  (locals (LocalClass :type "/Game/Blueprint/QuestActors/BP_MasterQuest Class Reference") (LocalStart :type Boolean) (LocalQuestActor :type "/Game/Blueprint/QuestActors/BP_MasterQuest Object Reference"))
  (bind _localquestactor (`local.LocalQuestActor`))
  (bind _mainwidget (`self.MainWidget`))
  (bind _localquestactor_2 (`local.LocalQuestActor`))
  (set `local.LocalClass` QuestClas)
  (set `local.LocalStart` `DirectlyStaert?`)
  (if (and (`KismetSystemLibrary.IsValidClass` QuestClas) (not (`KismetArrayLibrary.Array_Contains` (`self.AllQuestClasses`) QuestClas)))
    (`KismetArrayLibrary.Array_Add` (`self.AllQuestClasses`) (`local.LocalClass`))
    (bind _returnvalue (`|SpawnActorFromClass` (`local.LocalClass`) (`KismetMathLibrary.MakeTransform` (0.0 0.0 0.0)) "AlwaysSpawn" "OverrideRootScale" null self null null))
    (bind _output_get (set `local.LocalQuestActor` _returnvalue))
    (`KismetArrayLibrary.Array_Add` (`self.CurrentQuestActors`) _output_get)
    (bind _questwidget (`/Game/QuestSystem/Widgets/W_MainWidget.AddQuestToList` (`self.MainWidget`) _localquestactor_2))
    (bind _output_get_2 (set `/Game/Blueprint/QuestActors/BP_MasterQuest.QuestWidget` _questwidget (`local.LocalQuestActor`)))
    (`/Game/Blueprint/QuestActors/BP_MasterQuest.SetupStartingGoals` _localquestactor_2)
    (`/Game/QuestSystem/Widgets/W_QuestWidget.UpdateQuest` _output_get_2)
    (`/Game/QuestSystem/Widgets/W_QuestJournal.AddEntry` (`/Game/QuestSystem/Widgets/W_MainWidget.W_QuestJournal` (`self.MainWidget`)) (`local.LocalQuestActor`))
    (if (or (`local.LocalStart`) (<= (`KismetArrayLibrary.Array_Length` (`self.CurrentQuestActors`)) 1))
      (`self.SelectNewQuest` _localquestactor (`|GetArrayItem` (`/Game/QuestSystem/Widgets/W_QuestWidget.SubGoladWidget` (`/Game/Blueprint/QuestActors/BP_MasterQuest.QuestWidget` _localquestactor)))))
    (if (`/Game/QuestSystem/Widgets/W_MainWidget.SlideOut?` (`self.MainWidget`))
      (`UserWidget.PlayAnimation` _mainwidget (`/Game/QuestSystem/Widgets/W_MainWidget.SlideOut` _mainwidget) 0.0 1 "Reverse" 1.0 false)
      (set `/Game/QuestSystem/Widgets/W_MainWidget.SlideOut?` false _mainwidget)
      (return true)
      (else
        (return true)))
    (else
      (return false))))

(fn `CompleteGoals`
  (for _array_element (`self.IndecesToCompleteLater`)
    (`/Game/Blueprint/QuestActors/BP_MasterQuest.CompleteSubGoal` (break `/Game/QuestSystem/Structure/S_IndexToComplete` _array_element) (`.Index_5_EAC085ED4DEE24CF0DBD3F8644FCA35D` (break `/Game/QuestSystem/Structure/S_IndexToComplete` _array_element)) false))
  (return))

(fn `DistanceToGoal`
  (returns (Distance :type Integer))
  (bind (_returnvalue_x _returnvalue_y) (`KismetMathLibrary.BreakVector` (`self.K2_GetActorLocation` (`self.Player`))))
  (bind (_returnvalue_x_2 _returnvalue_y_2) (`KismetMathLibrary.BreakVector` (`self.K2_GetActorLocation` (`self.CurrentGoalACtor`))))
  (return (`KismetMathLibrary.Round` (/ (`KismetMathLibrary.VSize` (- (`KismetMathLibrary.MakeVector` _returnvalue_x _returnvalue_y) (`KismetMathLibrary.MakeVector` _returnvalue_x_2 _returnvalue_y_2))) 100.0))))

(fn `EndQuest`
  (params (Quest :type "/Game/Blueprint/QuestActors/BP_MasterQuest Object Reference"))
  (locals (LocalQuest :type "/Game/Blueprint/QuestActors/BP_MasterQuest Object Reference"))
  (bind _currentgoalactor (`self.CurrentGoalACtor`))
  (bind _player (`self.Player`))
  (bind _localquest (`local.LocalQuest`))
  (bind _output (`|GetArrayItem` (`self.CurrentQuestActors`)))
  (bind (_name _category _description _region _completeionreward) (break `/Game/QuestSystem/Structure/S_QuestInfo` (`/Game/Blueprint/QuestActors/BP_MasterQuest.QuestInfo` (`local.LocalQuest`))))
  (bind _output_get (set `local.LocalQuest` Quest))
  (`KismetArrayLibrary.Array_RemoveItem` (`self.CurrentQuestActors`) _output_get)
  (`KismetArrayLibrary.Array_Add` (select `/Game/QuestSystem/Enums/E_QuestStates` (`/Game/Blueprint/QuestActors/BP_MasterQuest.CurrentState` (`local.LocalQuest`)) :`NewEnumerator0` (`self.CurrentQuestActors`) :`NewEnumerator1` (`self.CompletedQuestActors`) :`NewEnumerator2` (`self.FailedQuestActors`)) _localquest)
  (`/Game/QuestSystem/Widgets/W_QuestJournal.AddEntry` (`/Game/QuestSystem/Widgets/W_MainWidget.W_QuestJournal` (`self.MainWidget`)) _localquest)
  (if (== (`local.LocalQuest`) (`self.CurrentQuest`))
    (set `self.CurrentQuest` null)
    (`/Engine/EditorBlueprintResources/StandardMacros.IsValid` _currentgoalactor
      (:`Is Valid`
        (`self.K2_DestroyActor` _currentgoalactor)
        (`Widget.SetVisibility` (`/Game/QuestSystem/Widgets/W_MainWidget.DistanceBorder` (`self.MainWidget`)) "Hidden")
        (`Widget.SetVisibility` (`/Game/QuestSystem/Widgets/W_MiniMap.DirectionArrow` (`/Game/QuestSystem/Widgets/W_MainWidget.W_MiniMap` (`self.MainWidget`))) "Hidden"))
      (:`Is Not Valid`
        _))
    (`/Engine/EditorBlueprintResources/StandardMacros.IsValid` _output
      (:`Is Valid`
        (`self.SelectNewQuest` _output (`|GetArrayItem` (`/Game/QuestSystem/Widgets/W_QuestWidget.SubGoladWidget` (`/Game/Blueprint/QuestActors/BP_MasterQuest.QuestWidget` _output)))))
      (:`Is Not Valid`
        _)))
  (if (`/Game/Blueprint/QuestActors/BP_MasterQuest.SelectedInJournal` (`local.LocalQuest`))
    (`/Game/QuestSystem/Widgets/W_QuestJournal.OnQuestClicked` (`/Game/QuestSystem/Widgets/W_MainWidget.W_QuestJournal` (`self.MainWidget`)) null))
  (if (`|EnumEquality` (`/Game/Blueprint/QuestActors/BP_MasterQuest.CurrentState` (`local.LocalQuest`)) "NewEnumerator1")
    (`/Game/FirstPersonBP/Blueprints/FirstPersonCharacter.AddExp` _player (break `/Game/QuestSystem/Structure/S_QuestReward` _completeionreward))
    (`/Game/FirstPersonBP/Blueprints/FirstPersonCharacter.SetPrestigeByRegion` _player (+ (`/Game/FirstPersonBP/Blueprints/FirstPersonCharacter.GetPrestigeByRegion` _player _region) (`.PrestigePoints_4_4449C2AC43176C3D95EF1FA857AD7F20` (break `/Game/QuestSystem/Structure/S_QuestReward` _completeionreward))) _region)
    (return)
    (else
      (return))))

(fn `HasCurrentQuest?`
  (params (Class :type "/Game/Blueprint/QuestActors/BP_MasterQuest Class Reference"))
  (returns (`Out?` :type Boolean) (QuestActor :type "/Game/Blueprint/QuestActors/BP_MasterQuest Object Reference"))
  (locals (LocalFoundQuest :type "/Game/Blueprint/QuestActors/BP_MasterQuest Object Reference"))
  (bind _localfoundquest (`local.LocalFoundQuest`))
  (for _array_element (`self.CurrentQuestActors`)
    (if (== Class (`GameplayStatics.GetObjectClass` _array_element))
      (set `local.LocalFoundQuest` _array_element)
      (break)))
  (`/Engine/EditorBlueprintResources/StandardMacros.IsValid` _localfoundquest
    (:`Is Valid`
      (return true _localfoundquest))
    (:`Is Not Valid`
      (return false null))))

(fn `SelectNewQuest`
  (params (Quest :type "/Game/Blueprint/QuestActors/BP_MasterQuest Object Reference") (Subgoal :type "/Game/QuestSystem/Widgets/W_SubGoalWidget Object Reference") (`Loaded?` :type Boolean))
  (bind _currentquest (`self.CurrentQuest`))
  (bind _questwidget (`/Game/Blueprint/QuestActors/BP_MasterQuest.QuestWidget` _currentquest))
  (`/Engine/EditorBlueprintResources/StandardMacros.IsValid` _currentquest
    (:`Is Valid`
      (`Widget.SetIsEnabled` (`/Game/QuestSystem/Widgets/W_QuestWidget.QuestName` _questwidget) false)
      (`/Game/QuestSystem/Widgets/W_QuestWidget.SelectSubGoal` _questwidget null false))
    (:`Is Not Valid`
      _))
  (bind _output_get (set `self.CurrentQuest` Quest))
  (`/Game/QuestSystem/Widgets/W_QuestWidget.OnQuestSelected` (`/Game/Blueprint/QuestActors/BP_MasterQuest.QuestWidget` _output_get) Subgoal `Loaded?`)
  (return))

(fn `UpdateDirectionArrow?`
  (bind (_returnvalue_roll _returnvalue_pitch _returnvalue_yaw) (`KismetMathLibrary.BreakRotator` (`KismetMathLibrary.FindLookAtRotation` (`self.K2_GetActorLocation` (`self.Player`)) (`self.K2_GetActorLocation` (`self.CurrentGoalACtor`)))))
  (`Widget.SetRenderTransformAngle` (`/Game/QuestSystem/Widgets/W_MiniMap.DirectionArrow` (`/Game/QuestSystem/Widgets/W_MainWidget.W_MiniMap` (`self.MainWidget`))) _returnvalue_yaw)
  (return))

(fn `UserConstructionScript`)