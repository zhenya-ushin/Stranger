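; Quest-system actor that respawns queued enemy classes at random reachable points within its RespawnRadius sphere.
; RespawnEnemy queues a class and delay, starting a half-second looping timer that counts delays down and clears itself once the queue empties.
; Expired entries spawn flagged as quest-giver, talk-to NPCs linked back to this actor.
; Queue removal uses the expired-list loop index, not the stored queue index, then decrements remaining stored indices.
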(event `RespawnEnemy`
  (params (RespawnInfo :type "/Game/QuestSystem/Structure/S_RespawnEnemy Structure"))
  (`KismetArrayLibrary.Array_Add` (`self.RespawnList`) RespawnInfo)
  (if (not (`KismetSystemLibrary.K2_IsValidTimerHandle` (`self.RespawnTimer`)))
    (bind _returnvalue (`KismetSystemLibrary.K2_SetTimerDelegate` (delegate `RespawnTick`) 0.5 true))
    (set `self.RespawnTimer` _returnvalue)))

(event `RespawnTick`
  (bind _indecisspawn (`self.IndecisSpawn`))
  (for (_array_element _array_index) (`self.RespawnList`)
    (bind _returnvalue (- (break `/Game/QuestSystem/Structure/S_RespawnEnemy` _array_element) 0.5))
    (if (> _returnvalue 0.0)
      (`KismetArrayLibrary.Array_Set` (`self.RespawnList`) _array_index (make `/Game/QuestSystem/Structure/S_RespawnEnemy` _returnvalue (`.Enemy_6_15E6192540D5E599F9CC0AA8D4FBDBB4` (break `/Game/QuestSystem/Structure/S_RespawnEnemy` _array_element))))
      (else
        (`KismetArrayLibrary.Array_Add` (`self.IndecisSpawn`) _array_index))))
  (for (_array_element_2 _array_index_2) (`self.IndecisSpawn`)
    (bind (_output_time _output_enemy) (break `/Game/QuestSystem/Structure/S_RespawnEnemy` (`|GetArrayItem` (`self.RespawnList`) _array_element_2)))
    (bind _returnvalue_2 (`|SpawnActorFromClass` _output_enemy (`KismetMathLibrary.MakeTransform` (`NavigationSystemV1.K2_GetRandomReachablePointInRadius` (`self.K2_GetActorLocation`) (`SphereComponent.SphereRadius` (`self.RespawnRadius`)) null null)) "AdjustIfPossibleButAlwaysSpawn" "OverrideRootScale" null "NameNPC" null))
    (set `/Game/Blueprint/AI_With_Markovs_chain/BP_MasterNPC.IsQuestGiver?` true _returnvalue_2)
    (set `/Game/Blueprint/AI_With_Markovs_chain/BP_MasterNPC.IsQuestNPCtoTalk?` true _returnvalue_2)
    (set `/Game/Blueprint/AI_With_Markovs_chain/BP_MasterNPC.RespawnActor` self _returnvalue_2)
    (`KismetArrayLibrary.Array_Remove` (`self.RespawnList`) _array_index_2)
    (for _index (range _array_index_2 (+ (`KismetArrayLibrary.Array_LastIndex` (`self.IndecisSpawn`)) 1))
      (`KismetArrayLibrary.Array_Set` _indecisspawn _index (- (`|GetArrayItem` _indecisspawn _index) 1))))
  (`KismetArrayLibrary.Array_Clear` (`self.IndecisSpawn`))
  (if (not (> (`KismetArrayLibrary.Array_Length` (`self.RespawnList`)) 0))
    (`KismetSystemLibrary.K2_ClearAndInvalidateTimerHandle` (`self.RespawnTimer`))))

(fn `UserConstructionScript`)