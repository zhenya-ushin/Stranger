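; BP_Capture is a scene-capture actor that renders brush hits on BP_MasterNPC characters as a UV unwrap for mesh painting.
; On start it publishes capture size and unwrap location to MPC_Global, clears RT_Capture after a short delay, and creates a dynamic M_Unwrap material.
; PaintChar temporarily swaps the NPC mesh's first material for the unwrap one, passes hit location and brush radius, captures the scene, then restores the original.
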(event `self.ReceiveBeginPlay`
  (`self.InitParam`
    (:`Out`
      (bind _returnvalue (`KismetMaterialLibrary.CreateDynamicMaterialInstance` "/Game/DrawSystem/M_Unwrap.M_Unwrap"))
      (set `self.UwrapMaterial` _returnvalue))))

(fn `PaintChar`
  (params (Actor :type "Actor Object Reference") (HitLocation :type "Vector Structure") (BrushRadius :type "Float (double-precision)"))
  (locals (MeshComp :type "SkeletalMeshComponent Object Reference") (OriginalMaterial :type "MaterialInterface Object Reference"))
  (bind _asbp_master_npc (cast `/Game/Blueprint/AI_With_Markovs_chain/BP_MasterNPC` Actor))
  (set `local.MeshComp` (`Character.Mesh` _asbp_master_npc))
  (`|ExecutionSequence`
    (:`then_0`
      (set `local.OriginalMaterial` (`PrimitiveComponent.GetMaterial` (`local.MeshComp`) 0))
      (`PrimitiveComponent.SetMaterial` (`local.MeshComp`) 0 (`self.UwrapMaterial`))
      (`KismetSystemLibrary.PrintString` "исходный материал сохранен"))
    (:`then_1`
      (`MaterialInstanceDynamic.SetVectorParameterValue` (`self.UwrapMaterial`) "HitLocation" (`KismetMathLibrary.Conv_VectorToLinearColor` (`local.HitLocation`)))
      (`MaterialInstanceDynamic.SetScalarParameterValue` (`self.UwrapMaterial`) "BrushRadius" (`local.BrushRadius`))
      (`KismetSystemLibrary.PrintString` "передаем точку пересечения и радиус кисти"))
    (:`then_2`
      (`SceneCaptureComponent2D.CaptureScene` (`self.SceneCaptureComponent2D`))
      (`PrimitiveComponent.SetMaterial` (`local.MeshComp`) 0 (`local.OriginalMaterial`))
      (`KismetSystemLibrary.PrintString` "Захватили развертку и пприменяем исходный материал"))))

(fn `UserConstructionScript`)