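; BP_MasterQuest is a quest actor that tracks one quest's active and completed subgoals, hunt counters and growing description.
; CompleteSubGoal records success or failure, fires empty OnGoalCompleted/OnGoalFailed hooks, then either ends the quest through QuestManager or branches into follow-up goal indices.
; AddGoalForIndex recursively auto-completes goals whose item is already in the player's inventory, otherwise creating their widgets.
; Index-aligned arrays link goals, counters and widgets, and changes update the journal directly.
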(event `OnGoalFailed`
  (params (GoalIndex :type Integer)))

(event `OnGoalCompleted`
  (params (GoalIndex :type Integer)))

(fn `AddGoalForIndex`
  (params (Index :type Integer))
  (locals (LocalIndex :type Integer))
  (bind _questwidget (`self.QuestWidget`))
  (bind _localindex (`local.LocalIndex`))
  (bind _goal (`self.GoalAtIndex` (`local.LocalIndex`)))
  (bind _goal_2 (`self.GoalAtIndex` _localindex))
  (bind (_type _customgoal_ _goaltext _addition _amounttohunt _goalclass _taggoal _npcname _goalid _goallocation _useradius_ _radius _circlecolour _updatequestdesc_ _updateddescription) (break `/Game/QuestSystem/Structure/S_GoalInfo` _goal_2))
  (bind _output_get (set `local.LocalIndex` Index))
  (if (`self.GoalAlreadyFound?` _output_get)
    (`KismetArrayLibrary.Array_Add` (`self.CompletedSubGoals`) (make `/Game/QuestSystem/Structure/S_CompletedGoal` _localindex _goal_2 true))
    (`self.OnGoalCompleted` (`local.LocalIndex`))
    (if _updatequestdesc_
      (set `self.CurentDesc` (`|FormatText` "{Current}{Next}" (`self.CurentDesc`) _updateddescription))
      (if (`self.SelectedInJournal`)
        (`/Game/QuestSystem/Widgets/W_QuestJournal.UpdateDesc` (`/Game/QuestSystem/Widgets/W_MainWidget.W_QuestJournal` (`/Game/QuestSystem/Actors/BP_QuestManager.MainWidget` (`self.QuestManager`))))))
    (for _array_element (`.SubGoalIndecies_30_DAFB4D65488DD8C9BF49F1A662613694` (break `/Game/QuestSystem/Structure/S_GoalInfo` _goal_2))
      (`self.AddGoalForIndex` _array_element))
    (return)
    (else
      (bind _returnvalue (`KismetArrayLibrary.Array_Add` (`self.CurrentGoalIndecies`) (`local.LocalIndex`)))
      (if (> _returnvalue (`KismetArrayLibrary.Array_LastIndex` (`self.CurretHuntedAmounts`)))
        (`KismetArrayLibrary.Array_Add` (`self.CurretHuntedAmounts`)))
      (`KismetArrayLibrary.Array_Add` (`self.CurrentGoals`) _goal)
      (bind _returnvalue_2 (`|CreateWidget` "/Game/QuestSystem/Widgets/W_SubGoalWidget.W_SubGoalWidget_C" null _goal self (`self.QuestWidget`)))
      (`KismetArrayLibrary.Array_Add` (`/Game/QuestSystem/Widgets/W_QuestWidget.SubGoladWidget` _questwidget) _returnvalue_2)
      (`PanelWidget.AddChild` (`/Game/QuestSystem/Widgets/W_QuestWidget.SubGoal` _questwidget) _returnvalue_2)
      (return))))

(fn `CompleteSubGoal`
  (params (SubGoalIndeces :type Integer) (`Failed?` :type Boolean))
  (returns (Suc :type Boolean))
  (locals (LocalGoalIndex :type Integer) (LocalCompleteGoal :type "/Game/QuestSystem/Structure/S_GoalInfo Structure") (LocaWidgetIndex :type Integer :default 0) (`LocalFailed?` :type Boolean))
  (bind _questwidget (`self.QuestWidget`))
  (bind _localgoalindex (`local.LocalGoalIndex`))
  (bind _currentgoalindecies (`self.CurrentGoalIndecies`))
  (bind (_type _customgoal_ _goaltext _addition _amounttohunt _goalclass _taggoal _npcname _goalid _goallocation _useradius_ _radius _circlecolour _updatequestdesc_ _updateddescription) (break `/Game/QuestSystem/Structure/S_GoalInfo` (`local.LocalCompleteGoal`)))
  (bind (_type_2 _customgoal__2 _goaltext_2 _addition_2 _amounttohunt_2 _goalclass_2 _taggoal_2 _npcname_2 _goalid_2 _goallocation_2 _useradius__2 _radius_2 _circlecolour_2 _updatequestdesc__2 _updateddescription_2 _subgoalindecies _failmeansquestfail_ _completequest_) (break `/Game/QuestSystem/Structure/S_GoalInfo` (`local.LocalCompleteGoal`)))
  (bind _returnvalue (`KismetArrayLibrary.Array_Find` _currentgoalindecies (`local.LocalGoalIndex`)))
  (bind _subgoladwidget (`/Game/QuestSystem/Widgets/W_QuestWidget.SubGoladWidget` (`self.QuestWidget`)))
  (set `local.LocalFailed?` `Failed?`)
  (set `local.LocalGoalIndex` SubGoalIndeces)
  (if (`KismetArrayLibrary.Array_Contains` (`self.CurrentGoalIndecies`) (`local.LocalGoalIndex`))
    (bind _output_get (set `local.LocalCompleteGoal` (`|GetArrayItem` (`.SubGoals_24_0D709B5D4238C144508DD1B2EDE066F5` (break `/Game/QuestSystem/Structure/S_QuestInfo` (`self.QuestInfo`))) (`local.LocalGoalIndex`))))
    (`KismetArrayLibrary.Array_Add` (`self.CompletedSubGoals`) (make `/Game/QuestSystem/Structure/S_CompletedGoal` (`local.LocalGoalIndex`) _output_get (not (`local.LocalFailed?`))))
    (if (and _updatequestdesc_ (not (`local.LocalFailed?`)))
      (set `self.CurentDesc` (`|FormatText` "{Current}{Next}" (`self.CurentDesc`) _updateddescription))
      (if (`self.SelectedInJournal`)
        (`/Game/QuestSystem/Widgets/W_QuestJournal.UpdateDesc` (`/Game/QuestSystem/Widgets/W_MainWidget.W_QuestJournal` (`/Game/QuestSystem/Actors/BP_QuestManager.MainWidget` (`self.QuestManager`))))))
    (`KismetArrayLibrary.Array_RemoveItem` (`self.CurrentGoals`) (`local.LocalCompleteGoal`))
    (set `local.LocaWidgetIndex` _returnvalue)
    (`KismetArrayLibrary.Array_Remove` (`self.CurretHuntedAmounts`) _returnvalue)
    (`KismetArrayLibrary.Array_RemoveItem` _currentgoalindecies (`local.LocalGoalIndex`))
    (`Widget.RemoveFromParent` (`|GetArrayItem` _subgoladwidget (`local.LocaWidgetIndex`)))
    (`KismetArrayLibrary.Array_Remove` _subgoladwidget (`local.LocaWidgetIndex`))
    (if (`local.LocalFailed?`)
      (`self.OnGoalFailed` _localgoalindex)
      (if (`.FailMeansQuestFail?_54_647491AC463539019F7DE3B4E4FCCDF4` (break `/Game/QuestSystem/Structure/S_GoalInfo` (`local.LocalCompleteGoal`)))
        _
        (else
          (if (`self.SelectedInJournal`) :!label _label
            (`/Game/QuestSystem/Widgets/W_QuestJournal.GenerateSubGoals` (`/Game/QuestSystem/Widgets/W_MainWidget.W_QuestJournal` (`/Game/QuestSystem/Actors/BP_QuestManager.MainWidget` (`self.QuestManager`)))))
          (if (and (== (`local.LocalGoalIndex`) (`self.SelectedSubGoalIndex`)) (== (`/Game/QuestSystem/Actors/BP_QuestManager.CurrentQuest` (`self.QuestManager`)) self))
            (`/Game/QuestSystem/Widgets/W_QuestWidget.SelectSubGoal` _questwidget (`|GetArrayItem` (`/Game/QuestSystem/Widgets/W_QuestWidget.SubGoladWidget` _questwidget)) false)
            (return true)
            (else
              (return true)))))
      (else
        (`self.OnGoalCompleted` _localgoalindex)
        (if _completequest_
          _
          (else
            (for _array_element _subgoalindecies
              (`self.AddGoalForIndex` _array_element))
            (goto _label)))))
    (for _array_element_2 (`self.CurrentGoalIndecies`)
      (`KismetArrayLibrary.Array_Add` (`self.CompletedSubGoals`) (make `/Game/QuestSystem/Structure/S_CompletedGoal` _array_element_2 (`self.GoalAtIndex` _array_element_2))))
    (`KismetArrayLibrary.Array_Clear` (`self.CurrentGoalIndecies`))
    (`KismetArrayLibrary.Array_Clear` (`self.CurretHuntedAmounts`))
    (`KismetArrayLibrary.Array_Clear` (`self.CurrentGoals`))
    (set `self.CurrentState` (select `bool` (`local.LocalFailed?`) :`false` "NewEnumerator1" :`true` "NewEnumerator2" :!type "/Game/QuestSystem/Enums/E_QuestStates Enum"))
    (`Widget.RemoveFromParent` (`self.ListEntryWidget`))
    (`Widget.RemoveFromParent` (`self.QuestWidget`))
    (`/Game/QuestSystem/Actors/BP_QuestManager.EndQuest` (`self.QuestManager`) self)
    (return true)
    (else
      (return false))))

(fn `GoalAlreadyFound?`
  (params (GoalIndex :type Integer))
  (returns (`Out?` :type Boolean))
  (locals (LocalBool :type Boolean))
  (bind (_type _customgoal_ _goaltext _addition _amounttohunt _goalclass) (break `/Game/QuestSystem/Structure/S_GoalInfo` (`self.GoalAtIndex` GoalIndex)))
  (if (`|EnumEquality` _type "NewEnumerator2")
    (for _array_element (`.Inventory_5_93139C3945BF819BD28A21A0941488F0` (break `/Game/InventorySystem/S_Inventory` (`/Game/FirstPersonBP/Blueprints/FirstPersonCharacter.Inventory` (`/Game/QuestSystem/Actors/BP_QuestManager.Player` (`self.QuestManager`)))))
      (if (== _array_element _goalclass)
        (set `local.LocalBool` true)
        (break)))
    (return (`local.LocalBool`))
    (else
      (return false))))

(fn `GoalAtIndex`
  (params (Index :type Integer))
  (returns (Goal :type "/Game/QuestSystem/Structure/S_GoalInfo Structure"))
  (return (`|GetArrayItem` (`.SubGoals_24_0D709B5D4238C144508DD1B2EDE066F5` (break `/Game/QuestSystem/Structure/S_QuestInfo` (`self.QuestInfo`))) Index)))

(fn `GoToNextSubGoal`
  (returns (`Succ?` :type Boolean))
  (locals (NextIndex :type Integer :default 0))
  (bind _currentgoalindecies (`self.CurrentGoalIndecies`))
  (bind _returnvalue (+ (`.MaxValue` (`KismetMathLibrary.MaxOfIntArray` (`self.CurrentGoalIndecies`))) 1))
  (if (<= _returnvalue (`KismetArrayLibrary.Array_LastIndex` (`.SubGoals_24_0D709B5D4238C144508DD1B2EDE066F5` (break `/Game/QuestSystem/Structure/S_QuestInfo` (`self.QuestInfo`)))))
    (set `local.NextIndex` _returnvalue)
    (`KismetArrayLibrary.Array_Clear` _currentgoalindecies)
    (`KismetArrayLibrary.Array_Add` _currentgoalindecies (`local.NextIndex`))
    (`self.UpdateSubGoals`)
    (return true)
    (else
      (return false))))

(fn `SelectedInJournal`
  (returns (Out :type Boolean))
  (bind _selectedquest (`/Game/QuestSystem/Widgets/W_QuestJournal.SelectedQuest` (`/Game/QuestSystem/Widgets/W_MainWidget.W_QuestJournal` (`/Game/QuestSystem/Actors/BP_QuestManager.MainWidget` (`self.QuestManager`)))))
  (return (and (== _selectedquest self) (`KismetSystemLibrary.IsValid` _selectedquest))))

(fn `SetupStartingGoals`
  (`KismetArrayLibrary.Array_Clear` (`self.CurrentGoalIndecies`))
  (set `self.CurentDesc` (`.Description_8_58F773084001E101F2EC44A374A08CF8` (break `/Game/QuestSystem/Structure/S_QuestInfo` (`self.QuestInfo`))))
  (for _array_element (`self.StartingGoalIndecies`)
    (`self.AddGoalForIndex` _array_element))
  (`KismetArrayLibrary.Array_Resize` (`self.CurretHuntedAmounts`) (`KismetArrayLibrary.Array_Length` (`self.CurrentGoalIndecies`)))
  (`self.UpdateSubGoals`)
  (return))

(fn `UpdateSubGoals`
  (`KismetArrayLibrary.Array_Clear` (`self.CurrentGoals`))
  (for _array_element (`self.CurrentGoalIndecies`)
    (`KismetArrayLibrary.Array_Add` (`self.CurrentGoals`) (`|GetArrayItem` (`.SubGoals_24_0D709B5D4238C144508DD1B2EDE066F5` (break `/Game/QuestSystem/Structure/S_QuestInfo` (`self.QuestInfo`))) _array_element)))
  (return))

(fn `UserConstructionScript`)