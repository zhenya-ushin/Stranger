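; Main menu NPC that acts out a cigarette-smoking routine on its skeletal mesh.
; BeginPlay starts a looping seven-second timer that plays the get-cigarette animation on each tick.
; For the first five ticks, a DoN also fires the smoking animation, a debug counter print and the throw animation back-to-back without delays, so each animation immediately replaces the previous one.
; An unwired Timeline is left unused.
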(event `self.ReceiveBeginPlay`
  (`KismetSystemLibrary.K2_SetTimerDelegate` (delegate `AnimationSmock`) 7.0 true))

(event `AnimationSmock`
  (`SkeletalMeshComponent.PlayAnimation` (`self.Mesh`) "/Game/Characters/NPC/SmokingGuy/Animation/A_GetSigare.A_GetSigare" false)
  (bind _counter (`/Engine/EditorBlueprintResources/StandardMacros.Do N` 5)
    (:`Exit`
      (`SkeletalMeshComponent.PlayAnimation` (`self.Mesh`) "/Game/Characters/NPC/SmokingGuy/Animation/A_Smoking.A_Smoking" false)
      (`KismetSystemLibrary.PrintString` (`KismetStringLibrary.Conv_IntToString` _counter))
      (`SkeletalMeshComponent.PlayAnimation` (`self.Mesh`) "/Game/Characters/NPC/SmokingGuy/Animation/A_Trow.A_Trow" false))))

(fn `UserConstructionScript`)