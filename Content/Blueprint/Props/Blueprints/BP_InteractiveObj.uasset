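; Interactive prop the player can pick up, with a widget that shows its name and interaction prompt.
; Interact either adds its class to parallel inventory class/count arrays and destroys it, or attaches non-inventory types to the hand socket.
; An already held item is stowed, or destroyed and respawned by class before the camera.
; Save-interface loading restores the transform and destroys props not loaded; Throw and Using are empty.
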(event `DropItemIfNonInventory`
  (params (FPC_REf :type "/Game/FirstPersonBP/Blueprints/FirstPersonCharacter Object Reference"))
  (bind _firstpersoncamera (`/Game/FirstPersonBP/Blueprints/FirstPersonCharacter.FirstPersonCamera` FPC_REf))
  (`self.K2_DestroyActor` (`/Game/FirstPersonBP/Blueprints/FirstPersonCharacter.CurrentObjectInArm` FPC_REf))
  (`|SpawnActorFromClass` (`/Game/FirstPersonBP/Blueprints/FirstPersonCharacter.CurObjectInArmClassRef` FPC_REf) (`KismetMathLibrary.Conv_VectorToTransform` (+ (`SceneComponent.K2_GetComponentLocation` _firstpersoncamera) (* (`SceneComponent.GetForwardVector` _firstpersoncamera) 100.0))) "AdjustIfPossibleButDontSpawnIfColliding" "OverrideRootScale" null "" null))

(event `/Game/Blueprint/Props/Interfaces/BPI_Interaction.Interact`
  (params (AsFirstPersonCharacter :type "/Game/FirstPersonBP/Blueprints/FirstPersonCharacter Object Reference") (`SpawnFromInventory?` :type Boolean))
  (bind _currentobjectinarm (`/Game/FirstPersonBP/Blueprints/FirstPersonCharacter.CurrentObjectInArm` AsFirstPersonCharacter))
  (if (`|EnumInequality` (`self.TypeOfItem`) "NewEnumerator1")
    (`self.Add Item` AsFirstPersonCharacter self)
    (else
      (`PrimitiveComponent.SetCollisionResponseToAllChannels` (`self.Box`) "ECR_Ignore")
      (`PrimitiveComponent.SetSimulatePhysics` (`self.Box`) false)
      ;[1 1 1] Спавнить предмет в руке, а если предмет в руках то заспавнить на земле из рук
      (`KismetSystemLibrary.PrintString` "Этот предмет нельзя положить в инвентарь")
      (`/Engine/EditorBlueprintResources/StandardMacros.IsValid` _currentobjectinarm
        (:`Is Valid`
          (if (`|EnumInequality` (`/Game/Blueprint/Props/Blueprints/BP_InteractiveObj.TypeOfItem` _currentobjectinarm) "NewEnumerator1")
            (`self.Add Item` _currentobjectinarm AsFirstPersonCharacter _currentobjectinarm)
            (set `/Game/FirstPersonBP/Blueprints/FirstPersonCharacter.CurObjectInArmClassRef` (`GameplayStatics.GetObjectClass` self) AsFirstPersonCharacter :!label _label)
            (bind _output_get (set `/Game/FirstPersonBP/Blueprints/FirstPersonCharacter.CurrentObjectInArm` self AsFirstPersonCharacter))
            (`self.K2_AttachToComponent` _output_get (`Character.Mesh` AsFirstPersonCharacter) "RightArmSocket" "SnapToTarget" "SnapToTarget" "KeepRelative" true)
            (else
              (`self.DropItem` AsFirstPersonCharacter `SpawnFromInventory?`))))
        (:`Is Not Valid`
          (goto _label))))))

(event `self.ReceiveBeginPlay`
  (bind _asw_interact_widget (cast `/Game/QuestSystem/Widgets/W_InteractWidget` (`WidgetComponent.GetUserWidgetObject` (`self.Widget`))))
  (set `self.As W Interact Widget` _asw_interact_widget)
  (`TextBlock.SetText` (`/Game/QuestSystem/Widgets/W_InteractWidget.Name` _asw_interact_widget) (`self.Name`))
  (`self.HideText`))

(event `Throw`
  (params (Location :type "Vector Structure")))

(event `Using`)

(event `/Game/Blueprint/Interfaces/BPI_SaveLoad.BPI_LoadState`
  (params (DefaultSaveLoadSlotName :type String) (FromSlot :type Integer) (s_SaveDataObject :type "/Game/SaveSystem/S_ObjectData Structure") (s_savedGameSlot :type "/Game/SaveSystem/S_SavedGameSlot Structure"))
  (`self.LoadActor` s_SaveDataObject))

(event `/Game/Blueprint/Interfaces/BPI_SaveLoad.BPI_SaveState`
  (params (DefaultSaveLoadSlotName :type String) (ToSlot :type Integer) (s_SaveGameSlot :type "/Game/SaveSystem/S_SavedGameSlot Structure")))

(event `/Game/Blueprint/Interfaces/BPI_SaveLoad.BPI_LoadDone`
  (`self.Load_Done`))

(event `ShowText`
  (bind _as_w_interact_widget (`self.As W Interact Widget`))
  (`Widget.SetVisibility` (`/Game/QuestSystem/Widgets/W_InteractWidget.Name` _as_w_interact_widget) "Visible")
  (`Widget.SetVisibility` (`/Game/QuestSystem/Widgets/W_InteractWidget.TextInteraction` _as_w_interact_widget) "Visible"))

(event `HideText`
  (bind _as_w_interact_widget (`self.As W Interact Widget`))
  (`Widget.SetVisibility` (`/Game/QuestSystem/Widgets/W_InteractWidget.Name` _as_w_interact_widget) "Hidden")
  (`Widget.SetVisibility` (`/Game/QuestSystem/Widgets/W_InteractWidget.TextInteraction` _as_w_interact_widget) "Hidden"))

(event `OnGameLoaded`
  (params (ManagerRef :type "/Game/QuestSystem/Actors/BP_QuestManager Object Reference"))
  (if (`KismetArrayLibrary.Array_Contains` (`.Inventory_5_93139C3945BF819BD28A21A0941488F0` (break `/Game/InventorySystem/S_Inventory` (`/Game/FirstPersonBP/Blueprints/FirstPersonCharacter.Inventory` (`/Game/QuestSystem/Actors/BP_QuestManager.Player` ManagerRef)))) (`GameplayStatics.GetObjectClass` self))
    _))

(fn `Add Item`
  (params (FPCRef :type "/Game/FirstPersonBP/Blueprints/FirstPersonCharacter Object Reference") (ObjRef :type "/Game/Blueprint/Props/Blueprints/BP_InteractiveObj Object Reference"))
  (bind _returnvalue (`GameplayStatics.GetObjectClass` ObjRef))
  (bind (_inventory_inventory _inventory_slotcount) (break `/Game/InventorySystem/S_Inventory` (`/Game/FirstPersonBP/Blueprints/FirstPersonCharacter.Inventory` FPCRef)))
  (bind _returnvalue_2 (`KismetArrayLibrary.Array_Find` _inventory_inventory _returnvalue))
  (if (`KismetArrayLibrary.Array_Contains` _inventory_inventory _returnvalue)
    (`KismetArrayLibrary.Array_Set` _inventory_slotcount _returnvalue_2 (+ (`|GetArrayItem` _inventory_slotcount _returnvalue_2) 1))
    (else
      (`KismetArrayLibrary.Array_Add` _inventory_inventory _returnvalue)
      (`KismetArrayLibrary.Array_Add` _inventory_slotcount 1)))
  (`self.K2_DestroyActor`)
  (return))

(fn `DestroySelf`
  (`self.K2_DestroyActor`))

(fn `DropItem`
  (params (FPC_REf :type "/Game/FirstPersonBP/Blueprints/FirstPersonCharacter Object Reference") (Condition :type Boolean))
  (if Condition
    (`self.DropItemIfNonInventory` FPC_REf)
    (return)
    (else
      (`self.DropItemIfNonInventory` FPC_REf)
      (bind _output_get (set `/Game/FirstPersonBP/Blueprints/FirstPersonCharacter.CurrentObjectInArm` self FPC_REf))
      (set `/Game/FirstPersonBP/Blueprints/FirstPersonCharacter.CurObjectInArmClassRef` (`GameplayStatics.GetObjectClass` _output_get) FPC_REf)
      (`self.K2_AttachToComponent` _output_get (`Character.Mesh` FPC_REf) "RightArmSocket" "SnapToTarget" "SnapToTarget" "KeepRelative" true)
      (`ActorComponent.K2_DestroyComponent` (`/Game/Blueprint/Props/Blueprints/BP_InteractiveObj.Widget` _output_get))
      (return))))

(fn `GetSaveLoadGameObject`
  (returns (SaveGameObject :type "/Game/SaveSystem/BP_SaveGame Object Reference"))
  (return null))

(fn `Load_Done`
  (if (not (`self.Loaded`))
    (`self.DestroySelf`)))

(fn `LoadActor`
  (params (SaveData :type "/Game/SaveSystem/S_ObjectData Structure"))
  (`SceneComponent.K2_SetWorldTransform` (`self.Box`) SaveData_ObjectTransform_2_F115187C4B17941E2491B19497D8ED8A false false)
  (set `self.Loaded` true)
  (set `self.NeedToLoad?` `SaveData_NeedToLoad?_8_3E0D2A984B75804FB03F08AB3916BF18`))

(fn `SaveState`
  (returns (ActorInfo :type "/Game/SaveSystem/S_ObjectData Structure"))
  (return (make `/Game/SaveSystem/S_ObjectData` (`SceneComponent.K2_GetComponentToWorld` (`self.StaticMesh`)) (`GameplayStatics.GetObjectClass` self))))

(fn `UserConstructionScript`)