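; BP_DrawComponent is a component that turns its owning StaticMeshActor into a drawable canvas.
; On BeginPlay, for each material slot it reads the original color, creates a render target cleared to that color, and assigns a canvas material instance that displays it.
; It also creates a brush material instance and stores references to the render target and materials.
; A LoadDraw event restores a saved material onto the first slot.
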(event `self.ReceiveBeginPlay`
  (bind _staticmeshcomponent (`StaticMeshActor.StaticMeshComponent` (`self.As Static Mesh Actor`)))
  (bind _asstatic_mesh_actor (cast `StaticMeshActor` (`self.GetOwner`)))
  (bind _output_get (set `self.As Static Mesh Actor` _asstatic_mesh_actor))
  (bind _staticmeshcomponent_2 (`StaticMeshActor.StaticMeshComponent` _output_get))
  (for (_array_element _array_index) (`MeshComponent.GetMaterials` _staticmeshcomponent_2)
    (bind _returnvalue (`PrimitiveComponent.CreateDynamicMaterialInstance` _staticmeshcomponent_2 _array_index _array_element "None"))
    (bind _returnvalue_2 (`MaterialInstanceDynamic.K2_GetVectorParameterValue` _returnvalue "Param"))
    (set `self.DefMatColor` _returnvalue_2)
    (`|ExecutionSequence`
      (:`then_0`
        (bind _returnvalue_3 (`KismetRenderingLibrary.CreateRenderTarget2D` 1024 1024 "RTF_RGBA16f" (`self.DefMatColor`)))
        (bind _output_get_2 (set `self.RenderTarget` _returnvalue_3))
        (`KismetRenderingLibrary.ClearRenderTarget2D` _output_get_2 (`self.DefMatColor`)))
      (:`then_1`
        (bind _returnvalue_4 (`KismetMaterialLibrary.CreateDynamicMaterialInstance` "/Game/DrawSystem/SecondTurn/M_CanvasTemple.M_CanvasTemple"))
        (`MaterialInstanceDynamic.SetTextureParameterValue` _returnvalue_4 "RenderTargetTexture" (`self.RenderTarget`))
        (`MaterialInstanceDynamic.SetVectorParameterValue` _returnvalue_4 "None" (`self.DefMatColor`))
        (`PrimitiveComponent.SetMaterial` _staticmeshcomponent _array_index _returnvalue_4)
        (set `self.DefaultMaterial` (`PrimitiveComponent.GetMaterial` _staticmeshcomponent 0)))
      (:`then_2`
        (bind _returnvalue_5 (`KismetMaterialLibrary.CreateDynamicMaterialInstance` "/Game/DrawSystem/SecondTurn/M_Brush.M_Brush"))
        (set `self.BrushMaterial` _returnvalue_5)))))

(event `/Game/Blueprint/Interfaces/BPI_SaveDraw.LoadDraw`
  (params (StaticObjRef :type "StaticMeshActor Object Reference") (LinearColor :type "LinearColor Structure") (RenderTarget :type "TextureRenderTarget2D Object Reference") (SavedMaterial :type "MaterialInterface Object Reference"))
  (bind _asstatic_mesh_actor (cast `StaticMeshActor` (`self.GetOwner`)))
  (`PrimitiveComponent.SetMaterial` (`StaticMeshActor.StaticMeshComponent` _asstatic_mesh_actor) 0 SavedMaterial))