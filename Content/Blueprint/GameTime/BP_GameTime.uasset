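; BP_GameTime is an in-game clock driven by a timeline whose play rate comes from Speed in the construction script.
; BeginPlay seeks the timeline to the configured start time, converted to fractional hours by SetNewTime.
; Tick turns the timeline's Seconds track into a Timespan and prints it as an on-screen clock.
; An hour-8 wake-up call to two AI characters exists but is unconnected.
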(event EventTick
  (params (DeltaSeconds :type Float%20%28single-precision%29))
  (Variables|Default|SetSeconds (stale _seconds))
  (bind _output_get (Variables|Default|SetTime (Math|Timespan|MakeTimespan 0 0 0 (Math|Float|Truncate (Variables|Default|GetSeconds)))))
  (Development|PrintString (Utilities|String|Append (Utilities|String|ToString(Integer) (.Hours (Math|Timespan|BreakTimespan _output_get))) " : " (Utilities|String|ToString(Integer) (.Minutes (Math|Timespan|BreakTimespan _output_get))) " : " (Utilities|String|ToString(Integer) (.Seconds (Math|Timespan|BreakTimespan _output_get)))) true true "(R=1.000000,G=0.038389,B=0.675073,A=1.000000)" 0.5))

(event EventBeginPlay
  (CallFunction|SetNewTime (Math|Timespan|MakeTimespan 0 (Variables|Default|GetHours) (Variables|Default|GetMinutes) (Variables|Default|GetSeconds_0))))

(fn ConstructionScript
  (Components|Timeline|SetPlayRate (Variables|Default|GetTimeline_0) (Variables|Default|GetSpeed)))

(fn SetNewTime
  (params (Time :type Timespan%20Structure))
  (bind (_days _hours _minutes _seconds) (Math|Timespan|BreakTimespan Time))
  (Components|Timeline|SetNewTime (Variables|Default|GetTimeline_0) (+ (Math|Conversions|ToFloat(Integer) _hours) (/ (+ (Math|Conversions|ToFloat(Integer) _minutes) (/ (Math|Conversions|ToFloat(Integer) _seconds) 6e+01)) 6e+01))))