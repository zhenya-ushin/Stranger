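; BP_Clock is a clock that displays the current game time as hours, minutes and seconds.
; On BeginPlay it finds and caches the first BP_GameTime actor in the level.
; Every Tick, while that reference is valid, it copies the Time values from BP_GameTime into separate Hours, Minutes and Seconds text elements.
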(event `self.ReceiveBeginPlay`
  (bind _outactors (`GameplayStatics.GetAllActorsOfClass` "/Game/Blueprint/GameTime/BP_GameTime.BP_GameTime_C"))
  (set `self.BPGameTime` (`|GetArrayItem` _outactors)))

(event `self.ReceiveTick`
  (params (DeltaSeconds :type "Float (single-precision)"))
  (bind _bpgametime (`self.BPGameTime`))
  (bind (_days _hours _minutes _seconds) (`KismetMathLibrary.BreakTimespan` (`/Game/Blueprint/GameTime/BP_GameTime.Time` _bpgametime)))
  (`/Engine/EditorBlueprintResources/StandardMacros.IsValid` _bpgametime
    (:`Is Valid`
      (`TextRenderComponent.K2_SetText` (`self.Hours`) (`KismetTextLibrary.Conv_IntToText` _hours))
      (`TextRenderComponent.K2_SetText` (`self.Minutes`) (`KismetTextLibrary.Conv_IntToText` _minutes))
      (`TextRenderComponent.K2_SetText` (`self.Seconds`) (`KismetTextLibrary.Conv_IntToText` _seconds)))))

(fn `UserConstructionScript`)