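; AI controller for BP_MasterFightNPC that patrols random navmesh points and fights the player in melee.
; Perception updates and sight re-checks choose between chasing the FirstPersonCharacter and resuming patrol.
; On reaching the player, a DoOnce-gated SelectAction uses BPLearnFight's predicted player action; block and dodge are placeholders redirecting to two montage attacks.
; Attacks turn the NPC, apply damage as the montage starts, then reset the gate and re-check sight.
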(event `self.ReceiveBeginPlay`
  (`KismetSystemLibrary.Delay` 0.2)
  (bind _asbp_master_fight_npc (cast `/Game/Blueprint/AI_With_Markovs_chain/BP_MasterFightNPC` (`self.K2_GetPawn`))
    (:`then`
      (bind _output_get (set `self.SelfNPC` _asbp_master_fight_npc))
      (`KismetSystemLibrary.PrintString` (`KismetStringLibrary.Concat_StrStr` "У контроллера _" (`KismetSystemLibrary.GetDisplayName` self) "_Перс это_" (`KismetSystemLibrary.GetDisplayName` _output_get)) true true (struct :`G` 0.66 :`B` 1.0 :`A` 1.0) 9999.0)
      (`self.PatrolActions`))
    (:`CastFailed`
      (`KismetSystemLibrary.PrintString` "каст неудачный"))))

(event `RotateToAttack`
  (params (SelfRef :type "/Game/Blueprint/AI_With_Markovs_chain/BP_MasterFightNPC Object Reference") (Actor :type "Actor Object Reference"))
  (`self.K2_SetActorRotation` SelfRef (`KismetMathLibrary.MakeRotator` 0.0 0.0 (.yaw (`KismetMathLibrary.FindLookAtRotation` (`self.K2_GetActorLocation` SelfRef) (`self.K2_GetActorLocation` Actor)))) false))

(event `self.AIPerception.OnPerceptionUpdated`
  (params (UpdatedActors :type "Array of Actor Object Reference (by ref)"))
  (bind _as_first_person_character (`self.As First Person Character`))
  (`KismetSystemLibrary.Delay` 0.2)
  (if (not (`/Game/Blueprint/AI_With_Markovs_chain/BP_MasterNPC.IsDead?` (`self.SelfNPC`)))
    (for _array_element UpdatedActors
      (bind _asfirst_person_character (cast `/Game/FirstPersonBP/Blueprints/FirstPersonCharacter` _array_element))
      (`KismetSystemLibrary.PrintString` "Вижу ГГ" true true (struct :`R` 0.620957 :`G` 0.002553 :`B` 1.0 :`A` 1.0) 5.0)
      (set `self.As First Person Character` _asfirst_person_character)
      (break))
    (`/Engine/EditorBlueprintResources/StandardMacros.IsValid` _as_first_person_character
      (:`Is Valid`
        (`self.CatchMainCharacter` _as_first_person_character))
      (:`Is Not Valid`
        (`KismetSystemLibrary.Delay` 2.0)
        (`self.PatrolActions`)))))

(event `CatchMainCharacter`
  (params (DetectedActor :type "Actor Object Reference"))
  (if (== (`KismetArrayLibrary.Array_Find` (`AIPerceptionComponent.GetCurrentlyPerceivedActors` (`self.AIPerception`) "/Script/AIModule.AISense_Sight") (`self.As First Person Character`)) -1)
    (`KismetSystemLibrary.PrintString` "Я ПЕРЕСТАЛ ВИДЕТЬ ИГРОКА")
    (set `self.bIsSeePlayer?` false)
    (else
      (`KismetSystemLibrary.PrintString` "Я ВИЭУ ИГРОКА")
      ;[1 1 1] Присоединить к BREAK FOR EACH loop
      (set `self.bIsSeePlayer?` true)))
  (`self.FightwGG`))

(event `self.AIPerception.OnTargetPerceptionUpdated`
  (params (Actor :type "Actor Object Reference") (Stimulus :type "AIStimulus Structure")))

(event `FightwGG`
  (if (`self.bIsSeePlayer?`)
    (`|AIMoveTo` (`self.SelfNPC`) (0.0 0.0 0.0) (`self.As First Person Character`) 10.0 true
      (:`OnSuccess`
        (`KismetSystemLibrary.PrintString` "Дошел до ГГ" true true (struct :`R` 0.620957 :`G` 0.002553 :`B` 1.0 :`A` 1.0) 5.0)
        (`self.ChooseStrategy4Fight` (`self.As First Person Character`))))
    (else
      (`KismetSystemLibrary.Delay` 2.0)
      (`self.PatrolActions`))))

(event `PatrolActions`
  (bind _selfnpc (`self.SelfNPC`))
  (`|AIMoveTo` _selfnpc (`NavigationSystemV1.K2_GetRandomLocationInNavigableRadius` (`self.K2_GetActorLocation` _selfnpc) 1000.0 null null) null 10.0
    (:`OnSuccess`
      (`KismetSystemLibrary.Delay` 2.0)
      (`self.CatchMainCharacter` (`self.As First Person Character`)))))

(event `UseDodge`)

(event `AttackOnEggs`
  (params (Actor :type "Actor Object Reference"))
  (bind _selfnpc (`self.SelfNPC`))
  (`self.RotateToAttack` (`self.SelfNPC`) Actor)
  (if (`/Game/Blueprint/AI_With_Markovs_chain/BP_MasterNPC.bIsAnimationPlaying?` _selfnpc)
    (`KismetSystemLibrary.Delay` 1.0))
  (`|PlayMontage` (`Character.Mesh` _selfnpc) "/Game/Characters/MC/Animation/RightArmAttack/Animation/AM_KickOnEggs.AM_KickOnEggs"
    (:`then`
      (`GameplayStatics.ApplyDamage` (`self.As First Person Character`) 6.0))
    (:`OnCompleted`
      (`self.ResetDoOnce` :!label _label)
      (`self.CatchMainCharacter` (`self.As First Person Character`)))
    (:`OnInterrupted`
      (goto _label))))

(event `AttackWarms`
  (params (Actor :type "Actor Object Reference"))
  (bind _selfnpc (`self.SelfNPC`))
  (`self.RotateToAttack` (`self.SelfNPC`) Actor)
  (if (`/Game/Blueprint/AI_With_Markovs_chain/BP_MasterNPC.bIsAnimationPlaying?` _selfnpc)
    (`KismetSystemLibrary.Delay` 1.0))
  (`|PlayMontage` (`Character.Mesh` _selfnpc) "/Game/Characters/MC/Animation/RightArmAttack/Animation/A_RightArmAttack1_Montage.A_RightArmAttack1_Montage"
    (:`then`
      (`GameplayStatics.ApplyDamage` (`self.As First Person Character`) 3.0))
    (:`OnCompleted`
      (`self.ResetDoOnce` :!label _label_2)
      (`self.CatchMainCharacter` (`self.As First Person Character`)))
    (:`OnInterrupted`
      (goto _label_2))))

(event `ResetDoOnce`
  (goto _label_3 :!via `Reset`))

(event `ChooseStrategy4Fight`
  (params (ActorVersus :type "Actor Object Reference"))
  ;[1 1 1] Обновляем DoOnce(мб пригодится когда нибудь)
  (`/Engine/EditorBlueprintResources/StandardMacros.DoOnce` false :!label _label_3
    (:`Completed`
      (`self.SelectAction` (select `int` (`/Game/GameComponents/BP_LearnAction.PredictedNextActionIndex` (`/Game/Blueprint/AI_With_Markovs_chain/BP_MasterNPC.BP_LearnFight` (`self.SelfNPC`))) :`0` 0 :`1` 1 :`2` 2 :`3` 3) ActorVersus))))

(fn `SelectAction`
  (params (ChoosenAction :type Integer) (ActorVersus :type "Actor Object Reference"))
  (`KismetSystemLibrary.PrintString` (`KismetStringLibrary.Concat_StrStr` "Игрок вероятно сделает действие №" (`KismetStringLibrary.Conv_IntToString` ChoosenAction)))
  (if (== ChoosenAction 0)
    (`KismetSystemLibrary.PrintString` (`KismetStringLibrary.Concat_StrStr` "Я собираюсь ставить блок"))
    (`self.SelectAction` 2 ActorVersus)
    (elif (== ChoosenAction 1)
      (`KismetSystemLibrary.PrintString` (`KismetStringLibrary.Concat_StrStr` "Я собираюсь уклоняться"))
      (`self.SelectAction` 3 ActorVersus)
      (elif (== ChoosenAction 2)
        (`self.AttackOnEggs` ActorVersus)
        (else
          ;[1 1 1] Добавить сюда последовательность тычек руками
          (`self.AttackWarms` ActorVersus))))))

(fn `UserConstructionScript`)