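; Base NPC Blueprint with health, interaction and health widgets, hit reactions, dialogue data and quest hooks.
; Melee hit reactions play montages, apply damage and increment counters on BP_LearnAction; hits from a specific interactive-item type also deal damage.
; Damage updates the health bar; death plays knockout montages, notifies the player and QuestManager, then destroys the actor.
; It spawns a head-attached BP_Capture, restores state from save slots and destroys itself if not loaded.
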(event `HitDecetionEggsKicking`
  ;[1 1 1] Реакция на удар по яйцам
  (if (not (`self.bIsKickOnEggsAMplaying?`))
    (set `self.bIsKickOnEggsAMplaying?` true)
    (set `self.bIsAnimationPlaying?` true)
    (`|PlayMontage` (`self.Mesh`) "/Game/Characters/NPC/Punk/Release/AM_ReactionKickEggs.AM_ReactionKickEggs"
      (:`then`
        (`/Game/GameComponents/BP_LearnAction.IncKeggs` (`self.BP_LearnFight`))
        (`GameplayStatics.ApplyDamage` self 15.0 null (`self.As First Person Character`)))
      (:`OnCompleted`
        (set `self.bIsKickOnEggsAMplaying?` false :!label _label)
        (set `self.bIsAnimationPlaying?` false))
      (:`OnInterrupted`
        (goto _label)))))

(event `HitDetectionRArm`
  (if (not (`self.bIsKickRarmAMplaying?`))
    (set `self.bIsKickRarmAMplaying?` true)
    (set `self.bIsAnimationPlaying?` true)
    (`|PlayMontage` (`self.Mesh`) "/Game/Characters/NPC/Punk/AM_Receive_Punch_To_The_FaceR.AM_Receive_Punch_To_The_FaceR"
      (:`then`
        (`/Game/GameComponents/BP_LearnAction.IncRarm` (`self.BP_LearnFight`))
        (`GameplayStatics.ApplyDamage` self 10.0 null (`self.As First Person Character`)))
      (:`OnCompleted`
        (set `self.bIsKickRarmAMplaying?` false :!label _label_2)
        (set `self.bIsAnimationPlaying?` false))
      (:`OnInterrupted`
        (goto _label_2)))))

(event `OnTalkWithQustNPC`
  (if (`self.IsQuestNPCtoTalk?`)
    (`/Game/QuestSystem/Actors/BP_QuestManager.OnTalkToNPC` (`/Game/FirstPersonBP/Blueprints/FirstPersonCharacter.QuestManager` (`self.As First Person Character`)) (`GameplayStatics.GetObjectClass` self) 0 (`self.NameNPC`))))

(event `HideTextEvent`
  (bind _interactwdget (`self.InteractWdget`))
  (`Widget.SetVisibility` (`/Game/QuestSystem/Widgets/W_InteractWidget.Name` _interactwdget) "Hidden")
  (`Widget.SetVisibility` (`/Game/QuestSystem/Widgets/W_InteractWidget.TextInteraction` _interactwdget) "Hidden"))

(event `ShowTextEvent`
  (bind _interactwdget (`self.InteractWdget`))
  (`Widget.SetVisibility` (`/Game/QuestSystem/Widgets/W_InteractWidget.Name` _interactwdget) "Visible")
  (`Widget.SetVisibility` (`/Game/QuestSystem/Widgets/W_InteractWidget.TextInteraction` _interactwdget) "Visible"))

(event `self.ReceiveBeginPlay`
  (bind (_returnvalue_x _returnvalue_y _returnvalue_z) (`KismetMathLibrary.BreakVector` (`SceneComponent.K2_GetComponentLocation` (`self.CapsuleComponent`))))
  (bind _returnvalue (`GameplayStatics.GetActorOfClass` "/Game/GameComponents/BP_LearnAction.BP_LearnAction_C"))
  (set `self.BP_LearnFight` _returnvalue)
  (`KismetSystemLibrary.Delay` 0.2)
  (bind _returnvalue_2 (`|SpawnActorFromClass` "/Game/DrawSystem/BP_Capture.BP_Capture_C" (`KismetMathLibrary.MakeTransform` (`KismetMathLibrary.MakeVector` _returnvalue_x _returnvalue_y (+ _returnvalue_z 90.0))) "AlwaysSpawn" "OverrideRootScale" null null))
  (`self.K2_AttachToComponent` _returnvalue_2 (`self.Mesh`) "Head" "KeepRelative" "KeepRelative" "KeepRelative" true)
  (set `self.BP_Capture` _returnvalue_2)
  (bind _asfirst_person_character (cast `/Game/FirstPersonBP/Blueprints/FirstPersonCharacter` (`GameplayStatics.GetPlayerCharacter` 0)))
  (set `self.As First Person Character` _asfirst_person_character)
  (bind _asw_interact_widget (cast `/Game/QuestSystem/Widgets/W_InteractWidget` (`WidgetComponent.GetUserWidgetObject` (`self.Widget`))))
  (bind _output_get (set `self.InteractWdget` _asw_interact_widget))
  (`TextBlock.SetText` (`/Game/QuestSystem/Widgets/W_InteractWidget.Name` _output_get) (`self.NameNPC`))
  (`self.HideTextEvent`)
  (bind _asw_enemys_health (cast `/Game/Blueprint/Widgets/W_EnemysHealth` (`WidgetComponent.GetUserWidgetObject` (`self.HealthWidget`))))
  (set `self.As W Enemys Health` _asw_enemys_health)
  (`self.UpdateHealth`)
  (bind _outactors (`GameplayStatics.GetAllActorsOfClass` "BP_MasterNPC_C"))
  (for (_array_element _array_index) _outactors
    (`KismetArrayLibrary.Array_Set` (`.Character_3_A968F77247FAFA5EC4FF69936F4776FA` (break `/Game/Blueprint/Struct/S_list_of_character` (`self.ListOfCharacters`))) _array_index _array_element true)))

(event `GiveQuest4GG`
  (params (NumberOfInput :type Integer)))

(event `self.ReceiveHit`
  (params (MyComp :type "PrimitiveComponent Object Reference") (Other :type "Actor Object Reference") (OtherComp :type "PrimitiveComponent Object Reference") (bSelfMoved :type Boolean) (HitLocation :type "Vector Structure") (HitNormal :type "Vector Structure") (NormalImpulse :type "Vector Structure") (Hit :type "HitResult Structure (by ref)"))
  (bind _asbp_interactive_obj (cast `/Game/Blueprint/Props/Blueprints/BP_InteractiveObj` Other))
  (if (`|EnumEquality` (`/Game/Blueprint/Props/Blueprints/BP_InteractiveObj.TypeOfItem` _asbp_interactive_obj) "NewEnumerator3")
    (`CharacterMovementComponent.DisableMovement` (`self.CharacterMovement`))
    (`KismetSystemLibrary.PrintString` "В меня попали")
    (`/Engine/EditorBlueprintResources/StandardMacros.DoOnce` false :!label _label_3
      (:`Completed`
        (`GameplayStatics.ApplyDamage` self 100.0 null (`self.As First Person Character`))))))

(event `self.ReceiveAnyDamage`
  (params (Damage :type "Float (single-precision)") (DamageType :type "DamageType Object Reference") (InstigatedBy :type "Controller Object Reference") (DamageCauser :type "Actor Object Reference"))
  (bind _output_get (set `self.DamageDiller` DamageCauser))
  (bind _output_get_2 (set `self.CurrentHealth` (- (`self.CurrentHealth`) (`KismetMathLibrary.FTrunc` Damage))))
  (`KismetSystemLibrary.PrintString` (`KismetStringLibrary.Conv_IntToString` _output_get_2))
  (`self.UpdateHealth`)
  (`self.CheckHealth`)
  (if (`self.IsDead?`)
    (`self.OnDeath` _output_get)
    (else
      (`KismetSystemLibrary.Delay` 0.1)
      (`CharacterMovementComponent.SetMovementMode` (`self.CharacterMovement`) "MOVE_Walking" 0)
      (`KismetSystemLibrary.PrintString` "иду дальше")
      (goto _label_3 :!via `Reset`))))

(event `OnDeath`
  (params (DamageDiller :type "Actor Object Reference"))
  (bind _as_first_person_character (`self.As First Person Character`))
  (bind _mesh (`self.Mesh`))
  (`MovementComponent.StopMovementImmediately` (`self.CharacterMovement`))
  (`|PlayMontage` _mesh "/Game/Characters/NPC/Punk/AM_Knocked_Out_Fall.AM_Knocked_Out_Fall"
    (:`OnCompleted`
      _)
    (:`OnInterrupted`
      _))
  (`|PlayMontage` _mesh "/Game/Characters/NPC/Punk/AM_Knocked_OutLOOP_.AM_Knocked_OutLOOP_"
    (:`then`
      _)
    (:`OnInterrupted`
      _))
  (`KismetSystemLibrary.PrintString` "Я умер")
  (`KismetSystemLibrary.PrintString` (`KismetStringLibrary.Concat_StrStr` "Меня убил_" (`KismetSystemLibrary.GetDisplayName` DamageDiller)))
  (`/Game/FirstPersonBP/Blueprints/FirstPersonCharacter.OnEnemyKilled` _as_first_person_character 50)
  ;[1 1 1] Мб пригодится для респавна
  (`/Game/QuestSystem/Actors/BP_QuestManager.OnEnemyKilled` (`/Game/FirstPersonBP/Blueprints/FirstPersonCharacter.QuestManager` _as_first_person_character) (`GameplayStatics.GetObjectClass` self))
  (set `self.NeedToLoad?` false)
  (`KismetSystemLibrary.Delay` 5.0)
  (`self.K2_DestroyActor`))

(event `OnOwnQuestCanceled`
  (params (Class :type "/Game/Blueprint/QuestActors/BP_MasterQuest Class Reference")))

(event `/Game/Blueprint/Interfaces/BPI_SaveLoadNPC.LoadDone`
  (if (not (`self.Loaded`))
    (`self.K2_DestroyActor` self)))

(event `/Game/Blueprint/Interfaces/BPI_SaveLoadNPC.LoadNPC`
  (params (SaveSlot :type "/Game/SaveSystem/S_NPCData Structure"))
  (`SceneComponent.K2_SetWorldTransform` (`self.CapsuleComponent`) SaveSlot_LocaionNPC_8_D5F28F8044B91AB97A24A5B89E31C4DC false false)
  (set `self.Loaded` true)
  (set `self.NameNPC` SaveSlot_NameNPC_50_5DC0D017450F0896D11EBB98435AFE3D)
  (`self.LoadDialogue` SaveSlot_DialogueTemp_22_87202E3B468B256FB0EA1491CA2D9AAB)
  (set `self.DialogueNumbers` SaveSlot_DialogueNumbers_33_4FBC12D9468C93E3F70B619A60084F2D)
  (set `self.NumberForGiveQuest` SaveSlot_NumberForGiveQuest_30_DFF23CB24E23D636FBFAC5AEBF728247)
  (set `self.CanSpeakWithAnyone` `SaveSlot_Can_Speak?_19_C5F329AE48C679C93DBB068EBF7228AD`)
  (set `self.IsQuestGiver?` `SaveSlot_IsQuestGiver?_25_E4E5DC7B45A8A1D4451D9C8B5F7743C5`)
  (set `self.IsQuestNPCtoTalk?` `SaveSlot_IsQuestNPCtoTALK?_34_28CDE771401F6E8C63F98592DF82DC25`)
  (set `self.RespawnActor` SaveSlot_RespawnActor_38_CDF1372541EAAB2F21DAABB2F56F64BE)
  (set `self.HasQuest` SaveSlot_HasQuest_41_96F2950D4AE13881FF6BCEA127466DF5)
  (set `self.CurrentHealth` SaveSlot_CurrentHealth_46_93C0FE86402E2A48DB2F059BD71B513A)
  (set `self.MaxHealth` SaveSlot_MaxHealth_47_99BC271047542019EBD03EA9FABA666D)
  (set `self.StartText4Dialogue` SaveSlot_StartDialogueText_54_B24B79054F3F6F8F865751B88D89A81D))

(event `/Game/Blueprint/Interfaces/BPI_SaveLoadNPC.SaveNPC`)

(fn `CheckHealth`
  (if (<= (`self.CurrentHealth`) 0)
    (`CharacterMovementComponent.DisableMovement` (`self.CharacterMovement`))
    (set `self.IsDead?` true)
    (return)
    (else
      (return))))

(fn `LoadDialogue`
  (params (S_DialogueTamlate :type "/Game/Blueprint/AI_With_Markovs_chain/S_DialogueTamlate Structure (by ref)"))
  (locals (LocalDialogueTemp :type "/Game/Blueprint/AI_With_Markovs_chain/S_DialogueTamlate Structure"))
  (bind _npcspeechpart1 (break `/Game/Blueprint/AI_With_Markovs_chain/S_NpcSpeech` (`.NpcSpeech_19_2F9A05A14FECC90F58AD09B115B758AA` (break `/Game/Blueprint/AI_With_Markovs_chain/S_DialogueTamlate` (`self.DialogueTemp`)))))
  (bind (_playerspeechpart1 _playerspeechpart2 _playerspeechadditional) (break `/Game/Blueprint/AI_With_Markovs_chain/S_PlayerSpeech` (`.PlayerSpeech_18_9096B795429FAFA012897A97B58DD005` (break `/Game/Blueprint/AI_With_Markovs_chain/S_DialogueTamlate` (`self.DialogueTemp`)))))
  (bind (_npcspeechpart1_2 _npcspeechpart2 _npcspeechadditional) (break `/Game/Blueprint/AI_With_Markovs_chain/S_NpcSpeech` (`.NpcSpeech_19_2F9A05A14FECC90F58AD09B115B758AA` (break `/Game/Blueprint/AI_With_Markovs_chain/S_DialogueTamlate` (`self.DialogueTemp`)))))
  (bind (_npcspeechpart1_3 _npcspeechpart2_2) (break `/Game/Blueprint/AI_With_Markovs_chain/S_NpcSpeech` (`.NpcSpeech_19_2F9A05A14FECC90F58AD09B115B758AA` (break `/Game/Blueprint/AI_With_Markovs_chain/S_DialogueTamlate` (`self.DialogueTemp`)))))
  (bind (_playerspeechpart1_2 _playerspeechpart2_2) (break `/Game/Blueprint/AI_With_Markovs_chain/S_PlayerSpeech` (`.PlayerSpeech_18_9096B795429FAFA012897A97B58DD005` (break `/Game/Blueprint/AI_With_Markovs_chain/S_DialogueTamlate` (`self.DialogueTemp`)))))
  (bind _output_get (set `local.LocalDialogueTemp` S_DialogueTamlate))
  ;[1 1 1] Заг8ружаем фразы персонажа
  (for (_ _array_index) _playerspeechpart1_2
    (bind (_playerspeechpart1_3 _playerspeechpart2_3) (break `/Game/Blueprint/AI_With_Markovs_chain/S_PlayerSpeech` (`.PlayerSpeech_18_9096B795429FAFA012897A97B58DD005` (break `/Game/Blueprint/AI_With_Markovs_chain/S_DialogueTamlate` _output_get))))
    (`KismetArrayLibrary.Array_Set` _playerspeechpart1_2 _array_index (`|GetArrayItem` _playerspeechpart1_3 _array_index)))
  (for (_ _array_index_2) _playerspeechpart2_2
    (`KismetArrayLibrary.Array_Set` _playerspeechpart2_2 _array_index_2 (`|GetArrayItem` _playerspeechpart2_3 _array_index_2)))
  (for (_ _array_index_3) _playerspeechadditional
    (`KismetArrayLibrary.Array_Set` _playerspeechadditional _array_index_3 (`|GetArrayItem` (`.PlayerSpeechAdditional_7_B07B032F46EC35DE8D14D4ABA5E98ECD` (break `/Game/Blueprint/AI_With_Markovs_chain/S_PlayerSpeech` (`.PlayerSpeech_18_9096B795429FAFA012897A97B58DD005` (break `/Game/Blueprint/AI_With_Markovs_chain/S_DialogueTamlate` (`local.LocalDialogueTemp`))))) _array_index_3)))
  (for (_ _array_index_4) _npcspeechpart1
    (`KismetArrayLibrary.Array_Set` _npcspeechpart1 _array_index_4 (`|GetArrayItem` (`.NpcSpeechPart1_3_72CAACC54FD35368788EB69DF84657E1` (break `/Game/Blueprint/AI_With_Markovs_chain/S_NpcSpeech` (`.NpcSpeech_19_2F9A05A14FECC90F58AD09B115B758AA` (break `/Game/Blueprint/AI_With_Markovs_chain/S_DialogueTamlate` (`local.LocalDialogueTemp`))))) _array_index_4)))
  (for (_ _array_index_5) _npcspeechpart2_2
    (`KismetArrayLibrary.Array_Set` _npcspeechpart2_2 _array_index_5 (`|GetArrayItem` (`.NpcSpeechPart2_5_4E2BF9D34198C522B0D2E5BF0A41CFB2` (break `/Game/Blueprint/AI_With_Markovs_chain/S_NpcSpeech` (`.NpcSpeech_19_2F9A05A14FECC90F58AD09B115B758AA` (break `/Game/Blueprint/AI_With_Markovs_chain/S_DialogueTamlate` (`local.LocalDialogueTemp`))))) _array_index_5)))
  (for (_ _array_index_6) _npcspeechadditional
    (`KismetArrayLibrary.Array_Set` _npcspeechadditional _array_index_6 (`|GetArrayItem` (`.NpcSpeechAdditional_7_37824AF54EAD7F68650AB88E552AC73A` (break `/Game/Blueprint/AI_With_Markovs_chain/S_NpcSpeech` (`.NpcSpeech_19_2F9A05A14FECC90F58AD09B115B758AA` (break `/Game/Blueprint/AI_With_Markovs_chain/S_DialogueTamlate` (`local.LocalDialogueTemp`))))) _array_index_6)))
  (return))

(fn `UpdateHealth`
  (bind _as_w_enemys_health (`self.As W Enemys Health`))
  (bind _currenthealth (`self.CurrentHealth`))
  (bind _maxhealth (`self.MaxHealth`))
  (`ProgressBar.SetPercent` (`/Game/Blueprint/Widgets/W_EnemysHealth.HealthBar` _as_w_enemys_health) (/ (`KismetMathLibrary.Conv_IntToDouble` _currenthealth) (`KismetMathLibrary.Conv_IntToDouble` _maxhealth)))
  (`TextBlock.SetText` (`/Game/Blueprint/Widgets/W_EnemysHealth.HealthText` _as_w_enemys_health) (`|FormatText` "{Current} / {Max}" (`KismetTextLibrary.Conv_IntToText` _currenthealth false false) (`KismetTextLibrary.Conv_IntToText` _maxhealth false false)))
  (return))

(fn `UserConstructionScript`)