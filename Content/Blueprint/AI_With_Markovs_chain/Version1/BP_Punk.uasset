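; BP_Punk is a punk NPC that talks to the player and can give or advance quests.
; It caches its AIC_ai_ver1_punk controller, which it notifies when logic or dialogue starts.
; Interaction halts movement, turns it toward the player and opens a dialogue widget.
; A matching input number grants its quest through the player's QuestManager and copies subgoal tags onto the player; tagged players also report talks there.
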(event `self.GiveQuest4GG`
  (params (NumberOfInput :type Integer))
  (`self.OnTalkWithQustNPC`)
  (if (`self.IsQuestGiver?`)
    (if (`KismetArrayLibrary.Array_Contains` (`/Game/QuestSystem/Actors/BP_QuestManager.AllQuestClasses` (`/Game/FirstPersonBP/Blueprints/FirstPersonCharacter.QuestManager` (`self.As First Person Character`))) (`self.HasQuest`))
      _
      (elif (== (`self.NumberForGiveQuest`) NumberOfInput)
        (`/Game/QuestSystem/Actors/BP_QuestManager.AddNewquest` (`/Game/FirstPersonBP/Blueprints/FirstPersonCharacter.QuestManager` (`self.As First Person Character`)) (`self.HasQuest`) true)
        (bind _returnvalue (`GameplayStatics.GetActorOfClass` (`self.HasQuest`)))
        (for _array_element (`.SubGoals_24_0D709B5D4238C144508DD1B2EDE066F5` (break `/Game/QuestSystem/Structure/S_QuestInfo` (`/Game/Blueprint/QuestActors/BP_MasterQuest.QuestInfo` _returnvalue)))
          (`KismetArrayLibrary.Array_Add` (`Actor.Tags` (`self.As First Person Character`)) (`.TagGoal_51_0F165A404EAF518D502CD7B66E7F8D71` (break `/Game/QuestSystem/Structure/S_GoalInfo` _array_element))))))))

(event `self.OnTalkWithQustNPC`
  (if (and (`self.ActorHasTag` (`self.As First Person Character`) (`self.TagToQuest`)) (`self.IsQuestNPCtoTalk?`))
    (`/Game/QuestSystem/Actors/BP_QuestManager.OnTalkToNPC` (`/Game/FirstPersonBP/Blueprints/FirstPersonCharacter.QuestManager` (`self.As First Person Character`)) (`GameplayStatics.GetObjectClass` self) 0 (`self.NameNPC`))))

(event `self.ReceiveBeginPlay`
  (`parent.ReceiveBeginPlay`)
  (bind _asaic_ai_ver_1_punk (cast `/Game/Blueprint/AI_With_Markovs_chain/Version1/AIC_ai_ver1_punk` (`self.GetController` self)))
  (bind _output_get (set `self.RefContoller` _asaic_ai_ver_1_punk))
  (`KismetSystemLibrary.PrintString` (`KismetStringLibrary.Concat_StrStr` "я_" (`KismetSystemLibrary.GetDisplayName` self) "_мой контроллер_" (`KismetSystemLibrary.GetDisplayName` _output_get)) true true (struct :`R` 0.708462 :`G` 0.076611 :`B` 1.0 :`A` 1.0) 999999.0))

(event `EventStartLogic`
  (`KismetSystemLibrary.Delay` 1e-05)
  (`/Game/Blueprint/AI_With_Markovs_chain/Version1/AIC_ai_ver1_punk.event_start_logic` (`self.RefContoller`))
  (set `self.CanSpeakWithAnyone` true))

(event `BPI_SaveState`
  (params (DefaultSaveLoadSlotName :type String) (ToSlot :type Integer) (s_SaveGameSlot :type "/Game/SaveSystem/S_SavedGameSlot Structure")))

(event `/Game/DialogueSystem/BPI_DialogueInterface4GG.StartInteraction`
  (params (GG :type "/Game/FirstPersonBP/Blueprints/FirstPersonCharacter Object Reference"))
  (`self.HideTextEvent`)
  (`KismetSystemLibrary.PrintString` "работает")
  (set `self.CanSpeakWithAnyone` false)
  (`/Game/Blueprint/AI_With_Markovs_chain/Version1/AIC_ai_ver1_punk.event_start_dialogue` (`self.RefContoller`))
  (`MovementComponent.StopMovementImmediately` (`self.CharacterMovement`))
  (bind _returnvalue (`|CreateWidget` "/Game/DialogueSystem/W_DialogueWith_BP_AI_ver1.W_DialogueWith_BP_AI_ver1_C" (`GameplayStatics.GetPlayerController` 0) null))
  (bind _output_get (set `self.DialogueWidget` _returnvalue))
  (`UserWidget.AddToViewport` _output_get 0)
  (set `/Game/DialogueSystem/W_DialogueWith_BP_AI_ver1.text1` (`self.StartText4Dialogue`) _output_get)
  (set `/Game/DialogueSystem/W_DialogueWith_BP_AI_ver1.RefChar` self _output_get)
  (`self.K2_SetActorRotation` (`KismetMathLibrary.MakeRotator` 0.0 0.0 (.yaw (`KismetMathLibrary.FindLookAtRotation` (`self.K2_GetActorLocation` self) (`self.K2_GetActorLocation` (`GameplayStatics.GetPlayerCharacter` 0)))))))

(fn `CanDialogWithOthers?`
  (returns (`CanSpeak?` :type Boolean))
  (return false))

(fn `GetSaveLoadGameObject`
  (returns (SaveGameObject :type "/Game/SaveSystem/BP_SaveGame Object Reference"))
  (return null))

(fn `UserConstructionScript`)