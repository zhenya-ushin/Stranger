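; Version 1 AI NPC pawn that the player can talk to and receive quests from.
; StartInteraction notifies AIC_ai_ver1, halts and turns the NPC toward the player, and opens a dialogue widget; startlogic restarts controller logic and re-enables talking.
; GiveQuest4GG reports talks to the QuestManager and, on a matching input number, adds the quest and tags the player with its subgoals.
; Random-state functions (working, cleaning, sleep, rain) are stubs.
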(event `self.ReceiveBeginPlay`
  ;[1 1 1] Получаем ссылку на контроллер
  (`parent.ReceiveBeginPlay`)
  (bind _asaic_ai_ver_1 (cast `/Game/Blueprint/AI_With_Markovs_chain/Version1/AIC_ai_ver1` (`self.GetController` self)))
  (bind _output_get (set `self.RefController` _asaic_ai_ver_1)))

(event `Move To Speak`
  (params (Punk :type "/Game/Blueprint/AI_With_Markovs_chain/Version1/BP_Punk Object Reference"))
  (`|AIMoveTo` (`self.RefController`) self (0.0 0.0 0.0) Punk 75.0
    (:`then`
      (`KismetSystemLibrary.PrintString` "Иду ебать" true true (struct :`R` 1.0 :`G` 0.963152 :`B` 0.086832 :`A` 1.0)))))

(event `Event start logic`
  (`KismetSystemLibrary.Delay` 1e-05)
  (`/Game/Blueprint/AI_With_Markovs_chain/Version1/AIC_ai_ver1.Event_start_logic` (`self.RefController`))
  (set `self.CanSpeakWithAnyone` true))

(event `self.GiveQuest4GG`
  (params (NumberOfInput :type Integer))
  (bind _as_first_person_character (`self.As First Person Character`))
  (`self.OnTalkWithQustNPC`)
  (if (`self.IsQuestGiver?`)
    (if (`KismetArrayLibrary.Array_Contains` (`/Game/QuestSystem/Actors/BP_QuestManager.AllQuestClasses` (`/Game/FirstPersonBP/Blueprints/FirstPersonCharacter.QuestManager` (`self.As First Person Character`))) (`self.HasQuest`))
      _
      (elif (== (`self.NumberForGiveQuest`) NumberOfInput)
        (`KismetSystemLibrary.PrintString` "БП ЕБЛАН ДАЮ КВЕСТ")
        (`/Game/QuestSystem/Actors/BP_QuestManager.AddNewquest` (`/Game/FirstPersonBP/Blueprints/FirstPersonCharacter.QuestManager` _as_first_person_character) (`self.HasQuest`) true)
        (bind _returnvalue (`GameplayStatics.GetActorOfClass` (`self.HasQuest`)))
        (for _array_element (`.SubGoals_24_0D709B5D4238C144508DD1B2EDE066F5` (break `/Game/QuestSystem/Structure/S_QuestInfo` (`/Game/Blueprint/QuestActors/BP_MasterQuest.QuestInfo` _returnvalue)))
          (`KismetArrayLibrary.Array_Add` (`Actor.Tags` _as_first_person_character) (`.TagGoal_51_0F165A404EAF518D502CD7B66E7F8D71` (break `/Game/QuestSystem/Structure/S_GoalInfo` _array_element))))))))

(event `/Game/DialogueSystem/BPI_DialogueInterface4GG.StartInteraction`
  (params (GG :type "/Game/FirstPersonBP/Blueprints/FirstPersonCharacter Object Reference"))
  (if (`self.CanSpeakWithAnyone`)
    (`self.HideTextEvent`)
    (`KismetSystemLibrary.PrintString` "работает")
    (set `self.CanSpeakWithAnyone` false)
    (`/Game/Blueprint/AI_With_Markovs_chain/Version1/AIC_ai_ver1.event_start_dialogue` (`self.RefController`))
    (`MovementComponent.StopMovementImmediately` (`self.CharacterMovement`))
    (bind _returnvalue (`|CreateWidget` "/Game/DialogueSystem/W_DialogueWith_BP_AI_ver1.W_DialogueWith_BP_AI_ver1_C" (`GameplayStatics.GetPlayerController` 0) null))
    (bind _output_get (set `self.DialogueWidget` _returnvalue))
    (`UserWidget.AddToViewport` _output_get 0)
    (set `/Game/DialogueSystem/W_DialogueWith_BP_AI_ver1.text1` (`self.StartText4Dialogue`) _output_get)
    (set `/Game/DialogueSystem/W_DialogueWith_BP_AI_ver1.RefChar` self _output_get)
    (`self.K2_SetActorRotation` (`KismetMathLibrary.MakeRotator` 0.0 0.0 (.yaw (`KismetMathLibrary.FindLookAtRotation` (`self.K2_GetActorLocation` self) (`self.K2_GetActorLocation` (`GameplayStatics.GetPlayerCharacter` 0))))))
    (else
      (`KismetSystemLibrary.PrintString` "Ща не могу разговаривать"))))

(event `Init`
  (params (DialogueArray :type "Array of Text (by ref)")))

(event `self.OnTalkWithQustNPC`
  (if (`self.IsQuestNPCtoTalk?`)
    (`/Game/QuestSystem/Actors/BP_QuestManager.OnTalkToNPC` (`/Game/FirstPersonBP/Blueprints/FirstPersonCharacter.QuestManager` (`self.As First Person Character`)) (`GameplayStatics.GetObjectClass` self) 0 (`self.NameNPC`))))

(fn `CheckOfRain`
  (params (VarForRain :type "Float (double-precision)"))
  (returns (`IsRainning?` :type Boolean))
  (return false))

(fn `Choose the State`
  (params (RandomVar :type "Float (double-precision)") (NumberOfWorkingState :type "Float (double-precision)") (NumberOfCleaning :type "Float (double-precision)") (NumberOfSleep :type "Float (double-precision)")))

(fn `DoThings`
  (params (NumberOfState :type Integer)))

(fn `Get Random Float`
  (params (`IsRainning?` :type Boolean) (Param2 :type Boolean)))

(fn `GetInit`
  (returns (InitArrayDialogue :type "Array of Text"))
  (return (`self.PlayerQuestionArray`)))

(fn `StateOfCleaning`)

(fn `StateOfSleep`)

(fn `StateOfWorking`)

(fn `UserConstructionScript`)