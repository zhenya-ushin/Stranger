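; Fight-learning component that records the player's arm hit, kick, block and dodge inputs to predict their next action.
; Each input runs UpdateInfo, which updates the current action's count row, keyed by previous action, and recomputes its ratios in a Markov-style table.
; The highest ratio's index becomes PredictedNextActionIndex, and UpdatePlayerData saves the row, resetting usage counters to 1.
; Frequency-based player typing and average attack timing are unconnected; debug prints trace each step.
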(event `IncRarm`
  (bind _s_playerinputinfight (`self.s_playerInputInFight`))
  (set `self.PrevActionIndex` (`self.CurActionIndex`) :!label _label)
  (bind _output_get (set `self.CurActionIndex` 0))
  (bind _result (`/Engine/EditorBlueprintResources/StandardMacros.IncrementInt` (`.CountOfUse_RightArm_23_70F68A484E5F2AE40303C6AAC92C3ED7` (break `/Game/GameComponents/S_PlayersInputInFight` _s_playerinputinfight)))
    (:`  `
      (`self.Update Info` _s_playerinputinfight _output_get)
      (`KismetSystemLibrary.PrintString` "Игрок Ударил Рукой"))))

(event `IncLarm`
  (goto _label))

(event `IncKeggs`
  (bind _s_playerinputinfight (`self.s_playerInputInFight`))
  (bind _result (`/Engine/EditorBlueprintResources/StandardMacros.IncrementInt` (`.CountOfUse_KickOnEggs_26_3339E66F45A5AD5CD475B192A30C4CAD` (break `/Game/GameComponents/S_PlayersInputInFight` _s_playerinputinfight)))
    (:`  `
      (`KismetSystemLibrary.PrintString` (`KismetStringLibrary.Conv_IntToString` _result))
      (set `self.PrevActionIndex` (`self.CurActionIndex`))
      (bind _output_get (set `self.CurActionIndex` 1))
      (`self.Update Info` _s_playerinputinfight _output_get)
      (`KismetSystemLibrary.PrintString` "Игрок Ударил ногой"))))

(event `IncDodge`
  (bind _s_playerinputinfight (`self.s_playerInputInFight`))
  (`/Engine/EditorBlueprintResources/StandardMacros.IncrementInt` (`.CountOfUse_Dodge_28_C29BDFD84795F8BC3B46E89F47B55F89` (break `/Game/GameComponents/S_PlayersInputInFight` _s_playerinputinfight))
    (:`  `
      (set `self.PrevActionIndex` (`self.CurActionIndex`))
      (bind _output_get (set `self.CurActionIndex` 3))
      (`self.Update Info` _s_playerinputinfight _output_get)
      (`KismetSystemLibrary.PrintString` "Игрок Увернулся"))))

(event `IncBblock`
  (bind _s_playerinputinfight (`self.s_playerInputInFight`))
  (`/Engine/EditorBlueprintResources/StandardMacros.IncrementInt` (`.CountOfUse_BodyBlock_27_E3D7C0B84CFEEB9F291C799D31780821` (break `/Game/GameComponents/S_PlayersInputInFight` _s_playerinputinfight))
    (:`  `
      (set `self.PrevActionIndex` (`self.CurActionIndex`))
      (bind _output_get (set `self.CurActionIndex` 2))
      (`self.Update Info` _s_playerinputinfight _output_get)
      (`KismetSystemLibrary.PrintString` "Игрок поставил блок"))))

(fn `GetMaxValueIndex`
  (params (FreqAvB :type "Float (double-precision)") (FreqAvD :type "Float (double-precision)") (FreqBvD :type "Float (double-precision)") (FreqArrayForFuture :type "Array of Float (double-precision)"))
  (returns (OptionIndex :type Integer))
  (locals (LocalMaxValue :type "Float (double-precision)") (SecondLocalMaxValue :type "Float (double-precision)") (LocalMaxIndex :type Integer))
  (bind _localmaxvalue (`local.LocalMaxValue`))
  (set `local.LocalMaxValue` (`|GetArrayItem` FreqArrayForFuture))
  (for (_array_element _array_index) FreqArrayForFuture
    (if (== _localmaxvalue _array_element)
      (set `local.SecondLocalMaxValue` _array_element)
      (elif (> _array_element _localmaxvalue)
        (set `local.LocalMaxIndex` _array_index)
        (set `local.LocalMaxValue` _array_element))))
  (if (== (`local.LocalMaxValue`) (`local.SecondLocalMaxValue`))
    (return 3)
    (else
      (return (`local.LocalMaxIndex`)))))

(fn `GetMaxValueProbability`
  (params (ProbabilityArray :type "Array of Float (double-precision)"))
  (returns (IndexAction :type Integer))
  (locals (LocalMaxIndex :type Integer) (LocalMaxValue :type "Float (double-precision)"))
  (set `local.LocalMaxValue` (`|GetArrayItem` ProbabilityArray))
  (set `local.LocalMaxIndex` 0)
  (for (_array_element _array_index) ProbabilityArray
    (if (> _array_element (`local.LocalMaxValue`))
      (set `local.LocalMaxValue` _array_element)
      (set `local.LocalMaxIndex` _array_index)))
  (return (`local.LocalMaxIndex`)))

(fn `GetProbability`
  (params (CurrentArrayActionProbability :type "Array of Float (double-precision)") (CurrentArrayActionCount :type "Array of Vector2D Structure"))
  (returns (UpdatedProbabilityArray :type "Array of Float (double-precision)"))
  (for (_array_element _array_index) CurrentArrayActionCount
    (bind (_x _y) (`KismetMathLibrary.BreakVector2D` _array_element))
    (`KismetArrayLibrary.Array_Set` CurrentArrayActionProbability _array_index (/ _x _y) true))
  (return (`self.CurrentActionProbabilityArray`)))

(fn `PredictNextAction`
  (params (CurrentActionProbabilityArray :type "Array of Float (double-precision)"))
  (bind _indexaction (`self.GetMaxValueProbability` CurrentActionProbabilityArray))
  (bind _output_get (set `self.PredictedNextActionIndex` _indexaction))
  (`KismetSystemLibrary.PrintString` (`KismetStringLibrary.Concat_StrStr` "Предсказанно действие №" (`KismetStringLibrary.Conv_IntToString` _output_get))))

(fn `Update Info`
  (params (S_PlayerInputInFight :type "/Game/GameComponents/S_PlayersInputInFight Structure") (CurrentActionIndex :type Integer))
  (bind (_countofuse_rightarm _countofuse_leftarm _countofuse_kickoneggs _countofuse_bodyblock _countofuse_dodge _avgtimebeforeplayerattacking _lastplayerattacktime _currentplayerattacktime _freqattackversusblock _freqattackversusdodge _freqblockversusdodge _subsequencecombo _0armattackarraycount _1legattackarraycount _2blockarraycount _3dodgearraycount _0armattackarrayprobability _1legattackarrayprobability _2blockarrayprobability _3dodgearrayprobability) (break `/Game/GameComponents/S_PlayersInputInFight` S_PlayerInputInFight))
  (`KismetSystemLibrary.PrintString` (`KismetStringLibrary.Concat_StrStr` "Игрок сделал действие_" (`KismetStringLibrary.Conv_IntToString` CurrentActionIndex)))
  (bind _output_get (set `self.CurrentActionCountArray` (select `int` (`self.CurActionIndex`) :`0` _0armattackarraycount :`1` _1legattackarraycount :`2` _2blockarraycount :`3` _3dodgearraycount)))
  (for (_array_element _array_index) _output_get
    (`KismetSystemLibrary.PrintString` (`KismetStringLibrary.Concat_StrStr` "Значения текущего массива счетчика действий: " "элемент№" (`KismetStringLibrary.Conv_IntToString` _array_index) "значение:" (`KismetStringLibrary.Conv_Vector2dToString` _array_element))))
  (bind _output_get_2 (set `self.CurrentActionProbabilityArray` (select `int` (`self.CurActionIndex`) :`0` _0armattackarrayprobability :`1` _1legattackarrayprobability :`2` _2blockarrayprobability :`3` _3dodgearrayprobability)))
  (for (_array_element_2 _array_index_2) _output_get_2
    (`KismetSystemLibrary.PrintString` (`KismetStringLibrary.Concat_StrStr` "Значения текущего массива вероятностей перехода: " "элемент№" (`KismetStringLibrary.Conv_IntToString` _array_index_2) "значение: " (`KismetStringLibrary.Conv_DoubleToString` _array_element_2))))
  (bind _updatedarray (`self.UpdateArray` _output_get))
  (bind _updatedprobabilityarray (`self.GetProbability` _output_get_2 _updatedarray))
  (`self.PredictNextAction` _updatedprobabilityarray)
  (`self.UpdatePlayerData` CurrentActionIndex _updatedprobabilityarray _updatedarray))

(fn `UpdateArray`
  (params (CurrentActionArray :type "Array of Vector2D Structure"))
  (returns (UpdatedArray :type "Array of Vector2D Structure"))
  (for (_array_element _array_index) CurrentActionArray
    (bind (_x _y) (`KismetMathLibrary.BreakVector2D` _array_element))
    (bind _result (`/Engine/EditorBlueprintResources/StandardMacros.IncrementFloat` _y)
      (:`  `
        (if (== _array_index (`self.PrevActionIndex`))
          (bind _result_2 (`/Engine/EditorBlueprintResources/StandardMacros.IncrementFloat` _x)
            (:`  `
              (`KismetArrayLibrary.Array_Set` CurrentActionArray _array_index (`KismetMathLibrary.MakeVector2D` _result_2 _result))))
          (else
            (`KismetArrayLibrary.Array_Set` CurrentActionArray _array_index (`KismetMathLibrary.MakeVector2D` _x _result)))))))
  (return (`self.CurrentActionCountArray`)))

(fn `UpdatePlayerData`
  (params (CurrentActionIndex :type Integer) (UpdatedProbabilityArray :type "Array of Float (double-precision)") (UpdatedActionCountArray :type "Array of Vector2D Structure"))
  (locals (ProbabilityLocalArray :type "Array of Float (double-precision)") (CountLocalArray :type "Array of Vector2D Structure"))
  (bind (_countofuse_rightarm _countofuse_leftarm _countofuse_kickoneggs _countofuse_bodyblock _countofuse_dodge _avgtimebeforeplayerattacking _lastplayerattacktime _currentplayerattacktime _freqattackversusblock _freqattackversusdodge _freqblockversusdodge _subsequencecombo _0armattackarraycount _1legattackarraycount _2blockarraycount _3dodgearraycount _0armattackarrayprobability _1legattackarrayprobability _2blockarrayprobability) (break `/Game/GameComponents/S_PlayersInputInFight` (`self.s_playerInputInFight`)))
  (bind (_countofuse_rightarm_2 _countofuse_leftarm_2 _countofuse_kickoneggs_2 _countofuse_bodyblock_2 _countofuse_dodge_2 _avgtimebeforeplayerattacking_2 _lastplayerattacktime_2 _currentplayerattacktime_2 _freqattackversusblock_2 _freqattackversusdodge_2 _freqblockversusdodge_2 _subsequencecombo_2 _0armattackarraycount_2 _1legattackarraycount_2 _2blockarraycount_2 _3dodgearraycount_2 _0armattackarrayprobability_2 _1legattackarrayprobability_2 _2blockarrayprobability_2 _3dodgearrayprobability) (break `/Game/GameComponents/S_PlayersInputInFight` (`self.s_playerInputInFight`)))
  (bind (_countofuse_rightarm_3 _countofuse_leftarm_3 _countofuse_kickoneggs_3 _countofuse_bodyblock_3 _countofuse_dodge_3 _avgtimebeforeplayerattacking_3 _lastplayerattacktime_3 _currentplayerattacktime_3 _freqattackversusblock_3 _freqattackversusdodge_3 _freqblockversusdodge_3 _subsequencecombo_3 _0armattackarraycount_3 _1legattackarraycount_3 _2blockarraycount_3 _3dodgearraycount_3 _0armattackarrayprobability_3 _1legattackarrayprobability_3 _2blockarrayprobability_3 _3dodgearrayprobability_2) (break `/Game/GameComponents/S_PlayersInputInFight` (`self.s_playerInputInFight`)))
  (bind (_countofuse_rightarm_4 _countofuse_leftarm_4 _countofuse_kickoneggs_4 _countofuse_bodyblock_4 _countofuse_dodge_4 _avgtimebeforeplayerattacking_4 _lastplayerattacktime_4 _currentplayerattacktime_4 _freqattackversusblock_4 _freqattackversusdodge_4 _freqblockversusdodge_4 _subsequencecombo_4 _0armattackarraycount_4 _1legattackarraycount_4 _2blockarraycount_4 _3dodgearraycount_4 _0armattackarrayprobability_4 _1legattackarrayprobability_4 _2blockarrayprobability_4 _3dodgearrayprobability_3) (break `/Game/GameComponents/S_PlayersInputInFight` (`self.s_playerInputInFight`)))
  (set `local.ProbabilityLocalArray` UpdatedProbabilityArray)
  (set `local.CountLocalArray` UpdatedActionCountArray)
  (if (== CurrentActionIndex 0)
    (set `self.s_playerInputInFight` (make `/Game/GameComponents/S_PlayersInputInFight` 1 1 1 1 1 0.0 0.0 0.0 0.0 0.0 0.0 0 (`local.CountLocalArray`) _1legattackarraycount_2 _2blockarraycount_2 _3dodgearraycount_2 (`local.ProbabilityLocalArray`) _1legattackarrayprobability_2 _2blockarrayprobability_2 _3dodgearrayprobability))
    (return)
    (elif (== CurrentActionIndex 1)
      (set `self.s_playerInputInFight` (make `/Game/GameComponents/S_PlayersInputInFight` 1 1 1 1 1 0.0 0.0 0.0 0.0 0.0 0.0 0 _0armattackarraycount_3 (`local.CountLocalArray`) _2blockarraycount_3 _3dodgearraycount_3 _0armattackarrayprobability_3 (`local.ProbabilityLocalArray`) _2blockarrayprobability_3 _3dodgearrayprobability_2))
      (return)
      (elif (== CurrentActionIndex 2)
        (set `self.s_playerInputInFight` (make `/Game/GameComponents/S_PlayersInputInFight` 1 1 1 1 1 0.0 0.0 0.0 0.0 0.0 0.0 0 _0armattackarraycount_4 _1legattackarraycount_4 (`local.CountLocalArray`) _3dodgearraycount_4 _0armattackarrayprobability_4 _1legattackarrayprobability_4 (`local.ProbabilityLocalArray`) _3dodgearrayprobability_3))
        (return)
        (else
          (set `self.s_playerInputInFight` (make `/Game/GameComponents/S_PlayersInputInFight` 1 1 1 1 1 0.0 0.0 0.0 0.0 0.0 0.0 0 _0armattackarraycount _1legattackarraycount _2blockarraycount (`local.CountLocalArray`) _0armattackarrayprobability _1legattackarrayprobability _2blockarrayprobability (`local.ProbabilityLocalArray`)))
          (return))))))

(fn `UserConstructionScript`)